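; Collectible component that registers its owning pickup with BP_GameInstance and handles one-time collection scoring.
; On the game instance's Initialize event, it records the owner's transform under a level, key and index tag if not yet initialized, then always destroys the owner.
; OnCollect adds Increment to the score, written to Spirit or otherwise Cherry, fires the collect event and removes the saved transform.
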(event Custom|InitializeEvent
  (bind _gameinstance (Variables|Default|GetGameInstance))
  (if (Variables|/Game/Game/Blueprints/GameInstance/BP_GameInstance.BP_GameInstance_C|GetIsInitialized _gameinstance)
    _
    (else
      (CallFunction|MakeTag)
      (Utilities|Map|Add (Variables|/Game/Game/Blueprints/GameInstance/BP_GameInstance.BP_GameInstance_C|GetTransformMap _gameinstance) (Variables|Default|GetTag) (Transformation|GetActorTransform (Components|GetOwner)))))
  (Actor|DestroyActor (Components|GetOwner)))

(event EventBeginPlay
  (bind _asbp_game_instance (Utilities|Casting|CastToBP_GameInstance (Game|GetGameInstance)))
  (bind _output_get (Variables|Default|SetGameInstance _asbp_game_instance))
  (EventDispatchers|BindEventtoInitialize _output_get (delegate Custom|InitializeEvent)))

(fn OnCollect
  (bind _gameinstance (Variables|Default|GetGameInstance))
  (bind _key (Variables|Default|GetKey))
  (bind _increment (Variables|Default|GetIncrement))
  (bind _key_2 (Variables|Default|GetKey))
  (bind _returnvalue (Utilities|Enum|Equal(Enum) _key_2 "Spirit"))
  (bind _scoremap (Variables|/Game/Game/Blueprints/GameInstance/BP_GameInstance.BP_GameInstance_C|GetScoreMap _gameinstance))
  (bind _value (Default|GetScorefromMap _gameinstance _key _scoremap))
  (bind _returnvalue_2 (select _returnvalue "Spirit" "Cherry"))
  (bind _returnvalue_3 (+ _value _increment))
  (if (not (Variables|Default|GetIsCollected))
    (Default|CallUpdateScore _gameinstance _returnvalue_2 _returnvalue_3)
    (Default|SetValue (Variables|Default|GetGameInstance) (Variables|/Game/Game/Blueprints/GameInstance/BP_GameInstance.BP_GameInstance_C|GetScoreMap (Variables|Default|GetGameInstance)) _returnvalue_2 _returnvalue_3)
    (Variables|Default|SetIsCollected true)
    (Default|CallCollectEvent)
    (CallFunction|MakeTag)
    (Utilities|Map|Remove (Variables|/Game/Game/Blueprints/GameInstance/BP_GameInstance.BP_GameInstance_C|GetTransformMap (Variables|Default|GetGameInstance)) (Variables|Default|GetTag))))

(fn MakeTag
  (bind _gameinstance (Variables|Default|GetGameInstance))
  (bind _returnvalue (Game|GetCurrentLevelName true))
  (Variables|Default|SetTag (Utilities|String|Append (Default|GetValuefromKey _gameinstance _returnvalue (Variables|/Game/Game/Blueprints/GameInstance/BP_GameInstance.BP_GameInstance_C|GetLevelMap _gameinstance)) (Variables|Default|GetKey) (Utilities|String|ToString(Integer) (Variables|Default|GetIndex)))))