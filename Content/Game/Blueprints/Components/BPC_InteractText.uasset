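; BPC_InteractText is a helper component that turns a child BP_DialogueStart into an "E" interact prompt.
; InitializeDialogueStart casts the given child actor, marks it autonomous, sets its dialogue creator text and resizes its widget.
; It then matches the dialogue's box to the supplied box's world transform and zeroes the widget's relative location.
; The event graph is inactive, with an unconnected call to that function.
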(event EventBeginPlay)

(event EventTick
  (params (DeltaSeconds :type Float%20%28single-precision%29)))

(fn InitializeDialogueStart
  (params (ChildActor :type Child%20Actor%20Component%20Object%20Reference) (Box :type Scene%20Component%20Object%20Reference))
  (bind _asbp_dialogue_start (Utilities|Casting|CastToBP_DialogueStart (Variables|/Script/Engine.ChildActorComponent|GetChildActor ChildActor)))
  (Variables|/Game/Game/Blueprints/Actors/BP_DialogueStart.BP_DialogueStart_C|SetAutonomous _asbp_dialogue_start true)
  (Variables|/Game/Game/Blueprints/Components/BPC_DialogueCreator.BPC_DialogueCreator_C|SetText (Variables|/Game/Game/Blueprints/Actors/BP_DialogueStart.BP_DialogueStart_C|GetBPC_DialogueCreator _asbp_dialogue_start) "E         ")
  (Class|WidgetComponent|SetDrawSize (Variables|/Game/Game/Blueprints/Actors/BP_DialogueStart.BP_DialogueStart_C|GetWidget _asbp_dialogue_start) "(X=100.000000,Y=100.000000)")
  (Transformation|SetWorldTransform (Variables|/Game/Game/Blueprints/Actors/BP_DetectionParent.BP_DetectionParent_C|GetBox _asbp_dialogue_start) (Transformation|GetWorldTransform Box) false false)
  (Transformation|SetRelativeLocation (Variables|/Game/Game/Blueprints/Actors/BP_DialogueStart.BP_DialogueStart_C|GetWidget _asbp_dialogue_start) "0, 0, 0" false false))