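; BP_Player is a player that moves in the YZ plane along arbitrarily angled surfaces, with a WhiteMode toggle that mirrors it across the surface.
; On ground, Tick averages a row of line traces to snap position and orientation to the surface.
; Jumping disables capsule collision and applies manual velocity and surface-relative gravity through the ground.
; In WhiteMode, sphere overlaps restore downward gravity on exit and reattach to BP_Wall using radial traces.
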(event OnComponentEndOverlap(Sphere)
  (params (OverlappedComponent :type Primitive%20Component%20Object%20Reference) (OtherActor :type Actor%20Object%20Reference) (OtherComp :type Primitive%20Component%20Object%20Reference) (OtherBodyIndex :type Integer))
  (Development|PrintString "End")
  (if (Variables|Default|GetWhiteMode)
    (if (and (!= OtherActor self) (Utilities|Array|IsEmpty (Collision|GetOverlappingActors (Variables|Default|GetSphere) "/Game/Game/Blueprints/BP_Wall.BP_Wall_C" :!class /Script/Engine.PrimitiveComponent)))
      (Variables|Default|SetGravityVector "0.000000,0.000000,-1.000000")
      (Variables|Default|SetIsInGround false))))

(event OnComponentBeginOverlap(Sphere)
  (params (OverlappedComponent :type Primitive%20Component%20Object%20Reference) (OtherActor :type Actor%20Object%20Reference) (OtherComp :type Primitive%20Component%20Object%20Reference) (OtherBodyIndex :type Integer) (bFromSweep :type Boolean) (SweepResult :type Hit%20Result%20Structure%20%28by%20ref%29))
  (bind _returnvalue (Transformation|GetActorLocation))
  (Development|PrintString "Begin")
  (if (Variables|Default|GetWhiteMode)
    (if (and (not (Variables|Default|GetIsInGround)) (not (Variables|Default|GetIsOnGround)))
      (Utilities|Casting|CastToBP_Wall OtherActor)
      (Variables|Default|SetIsOnGround true)
      (Utilities|FlowControl|Delay 0.0)
      (Variables|Default|SetLocation "0, 0, 0")
      (Variables|Default|SetUpVector "0, 0, 0")
      (Variables|Default|SetHitNumber 0)
      (for _index (range 0 360)
        (bind (_outhit _returnvalue_2) (Collision|LineTraceByChannel _returnvalue (+ _returnvalue (* (Math|Vector|RotateVectorAroundAxis "0.000000,0.000000,1.000000" (Math|Conversions|ToFloat(Integer) _index) "1.000000,0.000000,0.000000") 6e+01)) "TraceTypeQuery1" false 0 "None"))
        (if _returnvalue_2
          (Variables|Default|SetHitNumber (+ (Variables|Default|GetHitNumber) 1))
          (Variables|Default|SetLocation (+ (Variables|Default|GetLocation) (.Location (Collision|BreakHitResult _outhit))))
          (Variables|Default|SetUpVector (+ (Variables|Default|GetUpVector) (.Normal (Collision|BreakHitResult _outhit))))))
      (Transformation|SetWorldLocation (Variables|Default|GetCone) (Math|Vector|Lerp(Vector) (Transformation|GetActorLocation) (/ (Variables|Default|GetLocation) (Variables|Default|GetHitNumber)) 0.5) false false)
      (Transformation|SetWorldRotation (Variables|Default|GetCone) (Math|Rotator|MakeRotfromZX (/ (Variables|Default|GetUpVector) (Variables|Default|GetHitNumber)) (Math|Vector|MakeVector 1.0 0.0 0.0)) false false)
      (Transformation|SetWorldScale3D (Variables|Character|GetMesh) "0.255000,0.255000,0.255000"))))

(event Input|EnhancedActionEvents|EnhancedInputActionIA_Jump
  (params (ActionValue :type Boolean) (ElapsedSeconds :type Float%20%28double-precision%29) (TriggeredSeconds :type Float%20%28double-precision%29) (InputAction :type Input%20Action%20Object%20Reference :default "/Game/Game/Input/Actions/IA_Jump.IA_Jump"))
  (:Started
    (if (Variables|Default|GetIsOnGround)
      (Collision|SetCollisionEnabled (Variables|Collision|GetCapsuleComponent) "NoCollision")
      (if (Variables|Default|GetWhiteMode)
        (Variables|Default|SetVelocity (* (Variables|Default|GetUpVector) -0.5))
        (Variables|Default|SetIsOnGround false)
        (Variables|Default|SetIsInGround true)
        (Variables|Default|SetGravityVector (/ (Variables|Default|GetUpVector) 51.0))
        (else
          (Variables|Default|SetVelocity (* (Variables|Default|GetUpVector) 0.5))
          (Variables|Default|SetIsOnGround false)
          (Variables|Default|SetIsInGround true)
          (Variables|Default|SetGravityVector (/ (Variables|Default|GetUpVector) -51.0))
          (Transformation|SetActorLocation (Transformation|GetWorldLocation (Variables|Character|GetMesh)) false false))))))

(event Input|EnhancedActionEvents|EnhancedInputActionIA_Move
  (params (ActionValue :type Vector%202D%20Structure) (ElapsedSeconds :type Float%20%28double-precision%29) (TriggeredSeconds :type Float%20%28double-precision%29) (InputAction :type Input%20Action%20Object%20Reference :default "/Game/Game/Input/Actions/IA_Move.IA_Move"))
  (bind _returnvalue (Math|Vector|MakeVector 0.0 (.x ActionValue) (.y ActionValue)))
  (bind _deltatime (Variables|Default|GetDeltaTime))
  (bind _cone (Variables|Default|GetCone))
  (bind _cone_2 (Variables|Default|GetCone))
  (bind _mesh (Variables|Character|GetMesh))
  (bind _returnvalue_2 (Math|Vector|Normalize _returnvalue))
  (bind _returnvalue_3 (Math|Vector|GetRightVector _cone))
  (bind _returnvalue_4 (Math|Vector|GetUpVector _mesh))
  (bind _returnvalue_5 (Math|Vector|GetRightVector _cone_2))
  (bind _returnvalue_6 (* _deltatime 1e+01))
  (bind _returnvalue_7 (Math|Vector|DotProduct _returnvalue_2 _returnvalue_5))
  (bind _returnvalue_8 (* _returnvalue_4 102.0))
  (bind _returnvalue_9 (Math|Float|Sign(Float) _returnvalue_7))
  (bind _returnvalue_10 (Math|Float|Absolute(Float) _returnvalue_7))
  (bind _returnvalue_11 (- 1.0 _returnvalue_10))
  (bind _returnvalue_12 (Math|Float|Power _returnvalue_11 4.0))
  (bind _returnvalue_13 (- 1.0 _returnvalue_12))
  (bind _returnvalue_14 (* _returnvalue_9 _returnvalue_13))
  (bind _returnvalue_15 (* _returnvalue_3 _returnvalue_14))
  (bind _returnvalue_16 (* _returnvalue_15 _returnvalue_6))
  (:Triggered
    (Variables|Default|SetHorizontalVelocity (Math|Float|SelectFloat _returnvalue_14 (* _returnvalue_14 -1.0) (Variables|Default|GetWhiteMode)))
    (Transformation|SetActorLocation (Math|Vector|SelectVector (+ _returnvalue_16 (Transformation|GetActorLocation)) (+ (+ _returnvalue_16 (- (Transformation|GetActorLocation) _returnvalue_8)) _returnvalue_8) (Variables|Default|GetWhiteMode)) false false))
  (:Completed
    (Variables|Default|SetHorizontalVelocity 0.0)))

(event Input|EnhancedActionEvents|EnhancedInputActionIA_Swap
  (params (ActionValue :type Boolean) (ElapsedSeconds :type Float%20%28double-precision%29) (TriggeredSeconds :type Float%20%28double-precision%29) (InputAction :type Input%20Action%20Object%20Reference :default "/Game/Game/Input/Actions/IA_Swap.IA_Swap"))
  (:Started
    (Variables|Default|SetWhiteMode (not (Variables|Default|GetWhiteMode)))))

(event EventTick
  (params (DeltaSeconds :type Float%20%28single-precision%29))
  (bind _returnvalue (Transformation|GetActorLocation))
  (bind _mesh (Variables|Character|GetMesh))
  (bind _gravityvector (Variables|Default|GetGravityVector))
  (bind _mesh_2 (Variables|Character|GetMesh))
  (bind _cone (Variables|Default|GetCone))
  (bind _mesh_3 (Variables|Character|GetMesh))
  (Variables|Default|SetDeltaTime (* DeltaSeconds 75.0))
  (if (Variables|Default|GetIsOnGround)
    (Variables|Default|SetLocation "0, 0, 0")
    (Variables|Default|SetUpVector "0, 0, 0")
    (Variables|Default|SetAllHit true)
    (for _index (range 0 50)
      (bind (_location _up_vector _returnvalue_2) (CallFunction|LineTrace (+ _returnvalue (* (Math|Vector|GetRightVector _cone) (- _index 25))) (+ (- _returnvalue (* (Math|Vector|GetUpVector _cone) 1e+02)) (* (Math|Vector|GetRightVector _cone) (- _index 25)))))
      (Variables|Default|SetLocation (+ _location (Variables|Default|GetLocation)))
      (Variables|Default|SetUpVector (+ _up_vector (Variables|Default|GetUpVector)))
      (Variables|Default|SetAllHit (and _returnvalue_2 (Variables|Default|GetAllHit))))
    (if (Variables|Default|GetAllHit)
      (Transformation|SetActorLocation (Math|Vector|Lerp(Vector) (Transformation|GetActorLocation) (/ (Variables|Default|GetLocation) 51.0) 0.5) false false)
      (Transformation|SetWorldLocation (Variables|Default|GetCone) (Math|Vector|Lerp(Vector) (Transformation|GetActorLocation) (/ (Variables|Default|GetLocation) 51.0) 0.5) false false)
      (Transformation|SetWorldRotation (Variables|Default|GetCone) (Math|Rotator|MakeRotfromZX (/ (Variables|Default|GetUpVector) 51.0) (Math|Vector|MakeVector 1.0 0.0 0.0)) false false)
      (if (not (Variables|Default|GetWhiteMode))
        (Transformation|SetWorldLocation (Variables|Character|GetMesh) (+ (Transformation|GetWorldLocation _mesh_3) (* (Math|Vector|GetUpVector _mesh_3) -102.0)) false false)
        (Transformation|SetWorldRotation _mesh (Math|Rotator|MakeRotfromZX (Math|Vector|NegateVector (Math|Vector|GetUpVector _mesh)) (Math|Vector|MakeVector 1.0 0.0 0.0)) false false)))
    (else
      (Variables|Default|SetVelocity (+ (Variables|Default|GetVelocity) (* (Variables|Default|GetGravityVector) (Variables|Default|GetDeltaTime))))
      (Transformation|SetActorLocation (+ (Transformation|GetActorLocation) (* (Variables|Default|GetVelocity) (Variables|Default|GetDeltaTime))) false false)
      (Transformation|SetWorldLocation (Variables|Character|GetMesh) (+ (Transformation|GetActorLocation) (* (Variables|Default|GetVelocity) (Variables|Default|GetDeltaTime))) false false)
      (Transformation|SetWorldRotation (Variables|Default|GetCone) (Math|Rotator|MakeRotfromZX (select (Variables|Default|GetIsInGround) _gravityvector (Math|Vector|NegateVector _gravityvector)) (Math|Vector|MakeVector 1.0 0.0 0.0)) false false)
      (Transformation|SetWorldScale3D _mesh_2 (Math|Vector|Lerp(Vector) (Transformation|GetWorldScale _mesh_2) (select (Variables|Default|GetIsInGround) "0.255000,0.255000,-0.255000" "0.255000,0.255000,0.255000") 0.5)))))

(event EventBeginPlay
  (bind _asplayer_controller (Utilities|Casting|CastToPlayerController (Pawn|GetController)))
  (Utilities|IsValid (PlayerController|LocalPlayerSubsystems|GetEnhancedInputLocalPlayerSubsystem _asplayer_controller)
    (:Is%20Valid
      (Input|AddMappingContext (PlayerController|LocalPlayerSubsystems|GetEnhancedInputLocalPlayerSubsystem _asplayer_controller) "/Game/Game/Input/IMC_Default.IMC_Default" 0 "(bIgnoreAllPressedKeysUntilRelease=True,bForceImmediately=False,bNotifyUserSettings=False)"))))

(fn ConstructionScript)

(fn LineTrace
  (params (Start :type Vector) (End :type Vector))
  (bind (_outhit _returnvalue) (Collision|LineTraceByChannel Start End "TraceTypeQuery1" false 0 "None"))
  (return (+ (.Location (Collision|BreakHitResult _outhit)) (* (.Normal (Collision|BreakHitResult _outhit)) 51.0)) (.Normal (Collision|BreakHitResult _outhit)) _returnvalue))