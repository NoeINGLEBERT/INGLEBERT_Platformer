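; BP_Water is a water hazard volume that ends the run when a component tagged Player enters its box.
; The first such overlap fades music through BP_GameMode, plays a splash cue, nearly freezes time and shows a red "JIGOKU" level-transition widget given the current level's name.
; The construction script sizes a slightly tilted surface mesh and a cube to the box extents, applying a rotation parameter to a dynamic water material.
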(event OnComponentBeginOverlap(Box)
  (params (OverlappedComponent :type Primitive%20Component%20Object%20Reference) (OtherActor :type Actor%20Object%20Reference) (OtherComp :type Primitive%20Component%20Object%20Reference) (OtherBodyIndex :type Integer) (bFromSweep :type Boolean) (SweepResult :type Hit%20Result%20Structure%20%28by%20ref%29))
  (if (Components|ComponentHasTag OtherComp "Player")
    (Utilities|FlowControl|DoOnce false
      (:Completed
        (Default|FadeOutMusic (Variables|Default|GetGameMode))
        (Audio|PlaySound2D "/Game/Game/Audio/SoundCues/SC_Water.SC_Water" 1.0 1.0 0.0 0 0)
        (Utilities|FlowControl|Delay 0.01)
        (Utilities|Time|SetGlobalTimeDilation 0.02)
        (Utilities|FlowControl|Delay 0.01)
        (bind _returnvalue (Game|GetCurrentLevelName true))
        (bind _returnvalue_2 (UserInterface|CreateWidget "/Game/Game/Blueprints/Widgets/WBP_LevelTransition.WBP_LevelTransition_C" 0 "(R=1.000000,G=0.000000,B=0.000000,A=1.000000)" "JIGOKU" _returnvalue "(R=0.500000,G=0.500000,B=0.500000,A=1.000000)"))
        (UserInterface|Viewport|AddtoViewport _returnvalue_2 0)))))

(event EventBeginPlay
  (bind _asbp_game_mode (Utilities|Casting|CastToBP_GameMode (Game|GetGameMode)))
  (Variables|Default|SetGameMode _asbp_game_mode))

(fn ConstructionScript
  (bind _box (Variables|Default|GetBox))
  (bind _cube (Variables|Default|GetCube))
  (bind _box_2 (Variables|Default|GetBox))
  (bind _box_3 (Variables|Default|GetBox))
  (bind _returnvalue (Components|Box|GetScaledBoxExtent _box))
  (bind _returnvalue_2 (Transformation|GetWorldLocation _box_2))
  (bind _returnvalue_3 (Components|Box|GetScaledBoxExtent _box_3))
  (bind _returnvalue_4 (Transformation|GetWorldLocation _box_3))
  (bind (_x _y _z) (Math|Vector|BreakVector _returnvalue))
  (bind (_x_2 _y_2 _z_2) (Math|Vector|BreakVector _returnvalue_3))
  (bind (_x_3 _y_3 _z_3) (Math|Vector|BreakVector _returnvalue_4))
  (bind (_x_4 _y_4 _z_4) (Math|Vector|BreakVector _returnvalue_2))
  (bind _returnvalue_5 (+ _z_3 _z_2))
  (bind _returnvalue_6 (+ _x_3 _x_2))
  (bind _returnvalue_7 (- _x_3 _x_2))
  (bind _returnvalue_8 (Math|Vector|MakeVector _returnvalue_6 _y_3 _returnvalue_5))
  (bind _returnvalue_9 (- _returnvalue_5 6.5))
  (bind _returnvalue_10 (Math|Vector|MakeVector _returnvalue_7 _y_3 _returnvalue_9))
  (Transformation|SetWorldTransform (Variables|Default|GetStaticMesh) (Math|Transform|MakeTransform (Math|Vector|Lerp(Vector) _returnvalue_8 _returnvalue_10 0.5) (Math|Rotator|MakeRotfromXZ (Math|Vector|Normalize (- _returnvalue_8 _returnvalue_10)) (Math|Vector|MakeVector 0.0 0.0 1.0)) (Math|Vector|MakeVector (/ (Math|Vector|Distance(Vector) _returnvalue_8 _returnvalue_10) 1e+02) (/ _y_2 5e+01) 1.0)) false false)
  (bind _returnvalue_11 (Rendering|Material|CreateDynamicMaterialInstance (Variables|Default|GetStaticMesh) 0 "/Game/Game/Materials/Surface/M_WaterSurface.M_WaterSurface" "None" :!class /Script/Engine.PrimitiveComponent))
  (Rendering|Material|SetScalarParameterValue _returnvalue_11 "Rotation" (Variables|Default|GetMaterialRotation) :!class /Script/Engine.MaterialInstanceDynamic)
  (Transformation|SetWorldScale3D _cube (Math|Vector|MakeVector (/ _x 5e+01) (/ _y 5e+01) (/ (Math|Float|Max(Float) (- _z 13.0) 0.0) 5e+01)))
  (Transformation|SetWorldLocation _cube (Math|Vector|MakeVector _x_4 _y_4 (+ _z_4 (- (.Z (Math|Vector|BreakVector (Components|Box|GetScaledBoxExtent _box_2))) 6.5))) false false))