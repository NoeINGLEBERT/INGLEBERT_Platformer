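; Torii gate actor that serves as a level exit and player spawn point, with past/present-themed transition screens.
; When bound to the GameMode spawn event, it teleports the player, detaches the camera and auto-walks them out.
; Enter either starts departure (input lock, camera lock or zoom, auto-walk, music fade, transition widget) or, if input is disabled, eases the camera back and restores control.
; The construction script compensates component offsets for actor scale.
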(event OnComponentBeginOverlap(Box1)
  (params (OverlappedComponent :type Primitive%20Component%20Object%20Reference) (OtherActor :type Actor%20Object%20Reference) (OtherComp :type Primitive%20Component%20Object%20Reference) (OtherBodyIndex :type Integer) (bFromSweep :type Boolean) (SweepResult :type Hit%20Result%20Structure%20%28by%20ref%29))
  (if (Utilities|DoesObjectImplementInterface OtherActor "/Game/Game/Blueprints/Interfaces/BPI_Wave.BPI_Wave_C")
    (Class|BPIWave|Enter(Message) OtherActor)))

(event Custom|PlayCameraZoom
  (params (ZoomOut :type Boolean))
  (Variables|Default|SetStartArmLength (Variables|/Script/Engine.SpringArmComponent|GetTargetArmLength (Variables|/Game/Game/Blueprints/Actors/BP_Player.BP_Player_C|GetCameraBoom (Variables|Default|GetPlayer))))
  (if ZoomOut
    (bind (_direction _alpha) (Timeline|ZoomOut PlayFromStart)
      (:Update
        (bind _player (Variables|Default|GetPlayer)
          (:then
            (Variables|/Script/Engine.SpringArmComponent|SetTargetArmLength (Variables|/Game/Game/Blueprints/Actors/BP_Player.BP_Player_C|GetCameraBoom _player) (Math|Float|Lerp (Variables|Default|GetStartArmLength) (Utilities|Select :Index _direction :Forward 2.4e+03 :Backward 8e+02) _alpha)))
          (:else))))
    (else
      (Timeline|ZoomOut Reverse))))

(event Custom|TeleportPlayer
  (params (Index :type Integer))
  (bind _player (Variables|Default|GetPlayer))
  (bind _playerspawn (Variables|Default|GetPlayerSpawn))
  (bind _gameinstance (Variables|Default|GetGameInstance))
  (bind _returnvalue (Transformation|GetWorldTransform _playerspawn))
  (bind _followcamera (Variables|/Game/Game/Blueprints/Actors/BP_Player.BP_Player_C|GetFollowCamera _player))
  (if (== Index (Variables|Default|GetIndex))
    (Transformation|Teleport _player (.location _returnvalue) (.rotation _returnvalue))
    (Variables|/Script/Engine.SceneComponent|SetbAbsoluteLocation _followcamera true)
    (Transformation|SetWorldLocation _followcamera (Transformation|GetWorldLocation (Variables|Default|GetCameraSpawn)) false false)
    (Variables|/Game/Game/Blueprints/GameInstance/BP_GameInstance.BP_GameInstance_C|SetPlayerDirection _gameinstance (Math|Vector|DotProduct (Transformation|GetActorRightVector) "0.000000,1.000000,0.000000"))
    (Utilities|FlowControl|Delay 0.2)
    (Default|AutoMove (Variables|Default|GetPlayer) (Math|Vector2D|MakeVector2D (/ (Variables|/Game/Game/Blueprints/GameInstance/BP_GameInstance.BP_GameInstance_C|GetPlayerDirection _gameinstance) 2.0) 0.0) 1.0 1.67)))

(event EventBeginPlay
  (bind _asbp_game_mode (Utilities|Casting|CastToBP_GameMode (Game|GetGameMode)))
  (bind _output_get (Variables|Default|SetGameMode _asbp_game_mode))
  (Utilities|FlowControl|Delay 0.0)
  (Variables|Default|SetPlayer (Variables|/Game/Game/Blueprints/GameMode/BP_GameMode.BP_GameMode_C|GetPlayerRef _output_get))
  (bind _asbp_game_instance (Utilities|Casting|CastToBP_GameInstance (Game|GetGameInstance)))
  (Variables|Default|SetGameInstance _asbp_game_instance)
  (if (Variables|Default|GetIsSpawn)
    (EventDispatchers|BindEventtoSpawnPlayer (Variables|Default|GetGameMode) (delegate Custom|TeleportPlayer))))

(event EventEnter
  (bind _player (Variables|Default|GetPlayer))
  (bind _player_2 (Variables|Default|GetPlayer))
  (bind _ispast (Variables|Default|GetIsPast))
  (bind _returnvalue (Transformation|GetActorLocation _player))
  (bind _followcamera (Variables|/Game/Game/Blueprints/Actors/BP_Player.BP_Player_C|GetFollowCamera _player))
  (bind _followcamera_2 (Variables|/Game/Game/Blueprints/Actors/BP_Player.BP_Player_C|GetFollowCamera _player_2))
  (bind _returnvalue_2 (Transformation|GetWorldLocation _followcamera))
  (if (Variables|/Game/Game/Blueprints/GameMode/BP_GameMode.BP_GameMode_C|GetInputEnabled (Variables|Default|GetGameMode))
    (Input|DisableInput (Game|GetPlayerCharacter 0) (Game|GetPlayerController 0))
    (CallFunction|PlayCameraAnim)
    (Default|AutoMove (Variables|Default|GetPlayer) (Math|Vector2D|MakeVector2D (Math|Vector|DotProduct (Transformation|GetActorRightVector) "0.000000,-0.500000,0.000000") 0.0) (Variables|Default|GetAutoWalkSpeed) (Variables|Default|GetAutoWalkDuration))
    (if (Variables|Default|GetIsSpawn)
      (bind _returnvalue_3 (UserInterface|CreateWidget "/Game/Game/Blueprints/Widgets/WBP_Fade.WBP_Fade_C"))
      (UserInterface|Viewport|AddtoViewport _returnvalue_3 0)
      (Default|FadeOut _returnvalue_3)
      (Variables|/Game/Game/Blueprints/GameMode/BP_GameMode.BP_GameMode_C|SetInputEnabled (Variables|Default|GetGameMode) false)
      (Variables|/Game/Game/Blueprints/GameInstance/BP_GameInstance.BP_GameInstance_C|SetSpawnPoint (Variables|Default|GetGameInstance) (Variables|Default|GetIndex))
      (else
        (Audio|PlaySound2D "/Game/Game/Audio/SoundWaves/SW_Divine.SW_Divine" 1.0 1.0 0.0 0 0)))
    (Default|FadeOutMusic (Variables|Default|GetGameMode))
    (Utilities|FlowControl|Delay 1.25)
    (if (Variables|Default|GetIsSpawn)
      (bind _returnvalue_4 (UserInterface|CreateWidget "/Game/Game/Blueprints/Widgets/WBP_LevelTransition.WBP_LevelTransition_C" 0 (Math|Color|SelectColor "(R=0.000000,G=0.000000,B=0.000000,A=1.000000)" "(R=1.000000,G=1.000000,B=1.000000,A=1.000000)" _ispast) (Utilities|String|SelectText "MIRAI" "KAKO" _ispast) (Utilities|String|Append (Variables|Default|GetLevelName) (Utilities|String|SelectString "_1" "_0" _ispast)) (Math|Color|SelectColor "(R=4.000000,G=0.000000,B=0.000000,A=1.000000)" "(R=0.500000,G=0.500000,B=0.500000,A=1.000000)" _ispast)))
      (UserInterface|Viewport|AddtoViewport _returnvalue_4 0))
    (else
      (Utilities|FlowControl|Delay 0.1)
      (CallFunction|PlayCameraZoom false)
      (bind _alpha (Timeline|Timeline Play)
        (:Update
          (Transformation|SetWorldLocation _followcamera (Math|Vector|Lerp(Vector) (Math|Vector|MakeVector (.x _returnvalue_2) (.y _returnvalue_2) (.z _returnvalue_2)) (Math|Vector|MakeVector (.x _returnvalue_2) (.y _returnvalue) (.z _returnvalue)) _alpha) false false))
        (:Finished
          (Variables|/Script/Engine.SceneComponent|SetbAbsoluteLocation _followcamera_2 false)
          (Transformation|SetRelativeLocation _followcamera_2 "0, 0, 0" false false)
          (Input|EnableInput (Game|GetPlayerCharacter 0) (Game|GetPlayerController 0))
          (Variables|/Game/Game/Blueprints/GameMode/BP_GameMode.BP_GameMode_C|SetInputEnabled (Variables|Default|GetGameMode) true))))))

(fn ConstructionScript
  (Transformation|SetRelativeLocation (Variables|Default|GetBox1) (/ "0.000000,-1030.000000,80.000000" (Math|Vector|VectorGetAbs (Transformation|GetActorScale3D))) false false)
  (Transformation|SetRelativeLocation (Variables|Default|GetPlayerSpawn) (/ "0.000000,-1030.000000,52.000000" (Math|Vector|VectorGetAbs (Transformation|GetActorScale3D))) false false)
  (Transformation|SetRelativeLocation (Variables|Default|GetCameraSpawn) (/ "-800.000000,65.000000,50.000000" (Math|Vector|VectorGetAbs (Transformation|GetActorScale3D))) false false))

(fn PlayCameraAnim
  (bind _player (Variables|Default|GetPlayer))
  (bind _followcamera (Variables|/Game/Game/Blueprints/Actors/BP_Player.BP_Player_C|GetFollowCamera _player))
  (switch Utilities|FlowControl|Switch|SwitchonECameraAnim (Variables|Default|GetCameraAnim)
    (:NewEnumerator0
      (Transformation|SetRelativeLocation _followcamera (Transformation|GetWorldLocation _followcamera) false false)
      (Variables|/Script/Engine.SceneComponent|SetbAbsoluteLocation _followcamera true))
    (:NewEnumerator1
      (CallFunction|PlayCameraZoom true))))