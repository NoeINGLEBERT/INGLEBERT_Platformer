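; BP_SakuraTree is a tree that blooms when a visible actor overlaps its WaveDetection component and reverts when that actor leaves, unless locked.
; Each overlap change plays a sound and drives a timeline on the flowers' shared dynamic material Scale, while blooming also notifies the GameInstance.
; Construction randomizes flower rotation and scale, and an IsDead variant hides child actors, disabling their collision and Niagara auto-activation.
; GetState exposes whether it has flowers.
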(event OnComponentBeginOverlap(WaveDetection)
  (params (OverlappedComponent :type Primitive%20Component%20Object%20Reference) (OtherActor :type Actor%20Object%20Reference) (OtherComp :type Primitive%20Component%20Object%20Reference) (OtherBodyIndex :type Integer) (bFromSweep :type Boolean) (SweepResult :type Hit%20Result%20Structure%20%28by%20ref%29))
  (if (not (Variables|/Script/Engine.Actor|GetbHidden OtherActor))
    (Math|Integer|IncrementInt (Variables|Default|GetWaveInside)
      (:%20%20
        (Variables|Default|SetHasFlower true)
        (Default|CallSakuraActivate (Variables|Default|GetGameInstance))
        (Audio|PlaySoundatLocation "/Game/Game/Audio/SoundCues/SC_Sakura.SC_Sakura" (Transformation|GetActorLocation) "0, 0, 0" 0.5 2.0 0.0 0 0 0 0)
        (bind _alpha (Timeline|Timeline Play)
          (:Update
            (Rendering|Material|SetScalarParameterValue (Variables|Default|GetDynamicMaterial) "Scale" _alpha :!class /Script/Engine.MaterialInstanceDynamic)))))))

(event OnComponentEndOverlap(WaveDetection)
  (params (OverlappedComponent :type Primitive%20Component%20Object%20Reference) (OtherActor :type Actor%20Object%20Reference) (OtherComp :type Primitive%20Component%20Object%20Reference) (OtherBodyIndex :type Integer))
  (if (not (or (Variables|/Script/Engine.Actor|GetbHidden OtherActor) (Variables|Default|GetLocked)))
    (Math|Integer|DecrementInt (Variables|Default|GetWaveInside)
      (:%20%20
        (Variables|Default|SetHasFlower false)
        (Audio|PlaySoundatLocation "/Game/Game/Audio/SoundCues/SC_Sakura.SC_Sakura" (Transformation|GetActorLocation) "0, 0, 0" 0.25 2.0 0.0 0 0 0 0)
        (bind _alpha (Timeline|Timeline Reverse)
          (:Update
            (Rendering|Material|SetScalarParameterValue (Variables|Default|GetDynamicMaterial) "Scale" _alpha :!class /Script/Engine.MaterialInstanceDynamic)))))))

(event EventLock
  (Variables|Default|SetLocked true))

(event EventBeginPlay
  (bind _asbp_game_instance (Utilities|Casting|CastToBP_GameInstance (Game|GetGameInstance)))
  (Variables|Default|SetGameInstance _asbp_game_instance))

(fn ConstructionScript
  (bind _returnvalue (Math|Random|RandomFloatinRange 0.15 0.35))
  (Variables|Default|SetSakuraFlowers (Utilities|Array|MakeArray (Variables|Default|GetFlower0) (Variables|Default|GetFlower1) (Variables|Default|GetFlower2) (Variables|Default|GetFlower3) (Variables|Default|GetFlower4) (Variables|Default|GetFlower5) (Variables|Default|GetFlower6) (Variables|Default|GetFlower7) (Variables|Default|GetFlower8) (Variables|Default|GetFlower9) (Variables|Default|GetFlower10) (Variables|Default|GetFlower11) (Variables|Default|GetFlower12) (Variables|Default|GetFlower13)))
  (bind _returnvalue_2 (Rendering|Material|CreateDynamicMaterialInstance "/Game/Game/Materials/Surface/M_SakuraFlower.M_SakuraFlower" "None" "None" :!class /Script/Engine.KismetMaterialLibrary))
  (Variables|Default|SetDynamicMaterial _returnvalue_2)
  (for _array_element (Variables|Default|GetSakuraFlowers)
    (Rendering|Material|SetMaterial _array_element 0 (Variables|Default|GetDynamicMaterial))
    (Transformation|SetRelativeRotation _array_element (Math|Rotator|MakeRotator 9e+01 (Math|Random|RandomFloatinRange -1.8e+02 1.8e+02) 9e+01) false false)
    (Transformation|SetRelativeScale3D _array_element (Math|Vector|MakeVector _returnvalue _returnvalue _returnvalue)))
  (if (Variables|Default|GetIsDead)
    (for _array_element_2 (Utilities|Array|MakeArray (Variables|Default|GetChildActor) (Variables|Default|GetChildActor1) (Variables|Default|GetChildActor2) (Variables|Default|GetChildActor3) (Variables|Default|GetChildActor4) (Variables|Default|GetChildActor5))
      (Collision|SetActorEnableCollision (Variables|/Script/Engine.ChildActorComponent|GetChildActor _array_element_2) false)
      (Rendering|SetVisibility _array_element_2 false false))
    (Components|Activation|SetAutoActivate (Variables|Default|GetNiagara) false)))

(fn GetState
  (return (Variables|Default|GetHasFlower)))