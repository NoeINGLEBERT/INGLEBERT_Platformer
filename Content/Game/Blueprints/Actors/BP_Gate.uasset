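; BP_Gate is a level-transition gate that handles both leaving and what appears to be arriving, chosen by the GameMode's InputEnabled flag when Enter fires.
; With input enabled, it locks input, freezes the follow camera via absolute location, auto-moves the player, fades out and opens the target level.
; Otherwise, a Timeline pans the camera to the player's Y/Z, then restores relative following and input.
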(event EventBeginPlay
  (bind _asbp_game_mode (Utilities|Casting|CastToBP_GameMode (Game|GetGameMode)))
  (bind _output_get (Variables|Default|SetGameMode _asbp_game_mode))
  (Utilities|FlowControl|Delay 0.0)
  (Variables|Default|SetPlayer (Variables|/Game/Game/Blueprints/GameMode/BP_GameMode.BP_GameMode_C|GetPlayerRef _output_get)))

(event EventEnter
  (bind _player (Variables|Default|GetPlayer))
  (bind _player_2 (Variables|Default|GetPlayer))
  (bind _player_3 (Variables|Default|GetPlayer))
  (bind _returnvalue (Transformation|GetActorLocation _player_3))
  (bind _followcamera (Variables|/Game/Game/Blueprints/Actors/BP_Player.BP_Player_C|GetFollowCamera _player_3))
  (bind _followcamera_2 (Variables|/Game/Game/Blueprints/Actors/BP_Player.BP_Player_C|GetFollowCamera _player))
  (bind _followcamera_3 (Variables|/Game/Game/Blueprints/Actors/BP_Player.BP_Player_C|GetFollowCamera _player_2))
  (bind _returnvalue_2 (Transformation|GetWorldLocation _followcamera))
  (if (Variables|/Game/Game/Blueprints/GameMode/BP_GameMode.BP_GameMode_C|GetInputEnabled (Variables|Default|GetGameMode))
    (Input|DisableInput (Game|GetPlayerCharacter 0) (Game|GetPlayerController 0))
    (Transformation|SetRelativeLocation _followcamera_2 (Transformation|GetWorldLocation _followcamera_2) false false)
    (Variables|/Script/Engine.SceneComponent|SetbAbsoluteLocation _followcamera_2 true)
    (Default|AutoMove (Variables|Default|GetPlayer) "(X=-0.500000,Y=0.000000)")
    (bind _returnvalue_3 (UserInterface|CreateWidget "/Game/Game/Blueprints/Widgets/WBP_Fade.WBP_Fade_C"))
    (UserInterface|Viewport|AddtoViewport _returnvalue_3 0)
    (Default|FadeOut _returnvalue_3)
    (Variables|/Game/Game/Blueprints/GameMode/BP_GameMode.BP_GameMode_C|SetInputEnabled (Variables|Default|GetGameMode) false)
    (Utilities|FlowControl|Delay 1.25)
    (Game|OpenLevel(byObjectReference) (Variables|Default|GetLevel))
    (else
      (Utilities|FlowControl|Delay 0.1)
      (bind _alpha (Timeline|Timeline Play)
        (:Update
          (Transformation|SetWorldLocation _followcamera (Math|Vector|Lerp(Vector) (Math|Vector|MakeVector (.x _returnvalue_2) (.y _returnvalue_2) (.z _returnvalue_2)) (Math|Vector|MakeVector (.x _returnvalue_2) (.y _returnvalue) (.z _returnvalue)) _alpha) false false))
        (:Finished
          (Variables|/Script/Engine.SceneComponent|SetbAbsoluteLocation _followcamera_3 false)
          (Transformation|SetRelativeLocation _followcamera_3 "0, 0, 0" false false)
          (Input|EnableInput (Game|GetPlayerCharacter 0) (Game|GetPlayerController 0))
          (Variables|/Game/Game/Blueprints/GameMode/BP_GameMode.BP_GameMode_C|SetInputEnabled (Variables|Default|GetGameMode) true))))))

(fn ConstructionScript)