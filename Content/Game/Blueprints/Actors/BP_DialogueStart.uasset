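; Dialogue trigger actor that reveals configured text on a widget through BPCDialogueCreator when the player enters, playing a sound the first time.
; A timeline scaled to Duration drives the dialogue percentage and, with DoBlink, the post-process "Time" parameter.
; Autonomous instances restart the timeline on each entry and stop and clear the dialogue on exit; others just play it and ignore exit.
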(event EventPlayerLeaves
  (if (Variables|Default|GetAutonomous)
    (Utilities|FlowControl|Sequence
      (:then_0
        (bind _alpha (Timeline|Timeline Stop)
          (:Update
            (Default|SetDialogue (Variables|Default|GetBPC_DialogueCreator) (Variables|Default|GetWidget) _alpha)
            (if (Variables|Default|GetDoBlink)
              (Rendering|Material|SetScalarParameterValue "/Game/Game/Materials/ParameterCollection/MPC_PostProcess.MPC_PostProcess" "Time" _alpha :!class /Script/Engine.KismetMaterialLibrary)))))
      (:then_1
        (Default|SetDialogue (Variables|Default|GetBPC_DialogueCreator) (Variables|Default|GetWidget) 0.0)))))

(event EventPlayerEnters
  (Variables|Default|SetIsDisplayed true)
  (Utilities|FlowControl|Sequence
    (:then_0
      (if (Variables|Default|GetAutonomous)
        (bind _alpha (Timeline|Timeline PlayFromStart)
          (:Update
            (Default|SetDialogue (Variables|Default|GetBPC_DialogueCreator) (Variables|Default|GetWidget) _alpha)
            (if (Variables|Default|GetDoBlink)
              (Rendering|Material|SetScalarParameterValue "/Game/Game/Materials/ParameterCollection/MPC_PostProcess.MPC_PostProcess" "Time" _alpha :!class /Script/Engine.KismetMaterialLibrary))))
        (else
          (Timeline|Timeline Play))))
    (:then_1
      (Utilities|FlowControl|DoOnce false
        (:Completed
          (Audio|PlaySound2D (Variables|Default|GetSound) 1.0 1.0 0.0 0 0))))))

(fn ConstructionScript
  (bind _bpc_dialoguecreator (Variables|Default|GetBPC_DialogueCreator))
  (|CallParentFunction)
  (Variables|/Game/Game/Blueprints/Components/BPC_DialogueCreator.BPC_DialogueCreator_C|SetText _bpc_dialoguecreator (Variables|Default|GetText))
  (Variables|/Game/Game/Blueprints/Components/BPC_DialogueCreator.BPC_DialogueCreator_C|SetColor _bpc_dialoguecreator (Variables|Default|GetColor))
  (Components|Timeline|SetPlayRate (Variables|Default|GetTimeline) (/ 1.0 (Variables|Default|GetDuration))))