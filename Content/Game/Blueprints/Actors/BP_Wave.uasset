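; BP_Wave is a wave actor that travels along surfaces on a fixed X plane, scaling in and out with timelines.
; Each tick it averages a row of line traces to align with the surface and advance along its right vector.
; It saves its transform in the game instance under a level- and visibility-based tag, while Enter flips its facing and visibility.
; Overlapping an opposite-facing BPI_Wave actor reverses its spawn timeline.
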(event OnComponentBeginOverlap(Capsule)
  (params (OverlappedComponent :type Primitive%20Component%20Object%20Reference) (OtherActor :type Actor%20Object%20Reference) (OtherComp :type Primitive%20Component%20Object%20Reference) (OtherBodyIndex :type Integer) (bFromSweep :type Boolean) (SweepResult :type Hit%20Result%20Structure%20%28by%20ref%29))
  (if (and (Utilities|DoesObjectImplementInterface OtherActor "/Game/Game/Blueprints/Interfaces/BPI_Wave.BPI_Wave_C") (< (Math|Vector|DotProduct (Transformation|GetActorForwardVector OtherActor) (Transformation|GetActorForwardVector)) -0.8))
    (Utilities|FlowControl|Delay 0.0)
    (Transformation|SetActorRotation (Math|Rotator|MakeRotfromZY (Transformation|GetActorUpVector) (Math|Vector|MakeVector 1.0 0.0 0.0)))
    (CallFunction|Destroy)))

(event Custom|Destroy
  (bind _alpha (Timeline|Spawn Reverse)
    (:Update
      (Transformation|SetWorldScale3D (Variables|Default|GetWave) (Math|Vector|Lerp(Vector) "0, 0, 0" "0.750000,0.750000,0.750000" (Math|Float|Min(Float) (stale EventHide _alpha) _alpha))))
    (:Finished
      (if (< (.z (Transformation|GetWorldScale (Variables|Default|GetWave))) 0.1)
        (CallFunction|ClearSavedTransform)
        (Actor|DestroyActor)))))

(event EventEnter
  (Transformation|SetActorRotation (Math|Rotator|MakeRotfromZX (Transformation|GetActorUpVector) (Math|Vector|NegateVector (Transformation|GetActorForwardVector))))
  (Rendering|SetActorHiddenInGame (not (Variables|Rendering|GetbHidden))))

(event EventHide
  (Variables|Default|SetTargetSize (Transformation|GetWorldScale (Variables|Default|GetWave)))
  (Utilities|FlowControl|Sequence
    (:then_0
      (bind _alpha (Timeline|Timeline Reverse)
        (:Update
          (Transformation|SetWorldScale3D (Variables|Default|GetWave) (Math|Vector|Lerp(Vector) "0, 0, 0" (Variables|Default|GetTargetSize) _alpha)))))
    (:then_1
      (bind _alpha_2 (Timeline|Spawn Stop)
        (:Update
          (Transformation|SetWorldScale3D (Variables|Default|GetWave) (Math|Vector|Lerp(Vector) "0, 0, 0" "0.750000,0.750000,0.750000" (Math|Float|Min(Float) _alpha _alpha_2))))
        (:Finished
          (if (< (.z (Transformation|GetWorldScale (Variables|Default|GetWave))) 0.1)
            (CallFunction|ClearSavedTransform)
            (Actor|DestroyActor)))))))

(event EventTick
  (params (DeltaSeconds :type Float%20%28single-precision%29))
  (bind _returnvalue (Transformation|GetActorLocation))
  (bind _returnvalue_2 (Transformation|GetActorUpVector))
  (bind _returnvalue_3 (* _returnvalue_2 5e+01))
  (bind _returnvalue_4 (+ _returnvalue _returnvalue_3))
  (Variables|Default|SetLocation "0, 0, 0")
  (Variables|Default|SetUpVector "0, 0, 0")
  (Variables|Default|SetHitNumber 0)
  (for _index (range 0 50)
    (bind (_location _up_vector _returnvalue_5) (CallFunction|LineTrace (+ _returnvalue_4 (* (Transformation|GetActorRightVector) (- _index 25))) (+ (- _returnvalue_4 (* (Transformation|GetActorUpVector) 1e+02)) (* (Transformation|GetActorRightVector) (- _index 25)))))
    (if _returnvalue_5
      (Math|Integer|IncrementInt (Variables|Default|GetHitNumber)
        (:%20%20
          (Variables|Default|SetLocation (+ _location (Variables|Default|GetLocation)))
          (Variables|Default|SetUpVector (+ _up_vector (Variables|Default|GetUpVector)))))))
  (Transformation|SetActorRotation (Math|Rotator|MakeRotfromZX (/ (Variables|Default|GetUpVector) (Variables|Default|GetHitNumber)) (Transformation|GetActorForwardVector)))
  (Transformation|SetActorLocation (+ (/ (Variables|Default|GetLocation) (Variables|Default|GetHitNumber)) (* (Transformation|GetActorRightVector) (* DeltaSeconds 7.5e+02))) false false)
  (CallFunction|UpdateGameInstance))

(event EventBeginPlay
  (bind _asbp_game_instance (Utilities|Casting|CastToBP_GameInstance (Game|GetGameInstance)))
  (Variables|Default|SetGameInstance _asbp_game_instance)
  (Utilities|FlowControl|Sequence
    (:then_0
      (bind _alpha (Timeline|Timeline SetNewTime)
        (:Update
          (Transformation|SetWorldScale3D (Variables|Default|GetWave) (Math|Vector|Lerp(Vector) "0, 0, 0" (Variables|Default|GetTargetSize) _alpha)))))
    (:then_1
      (bind _alpha_2 (Timeline|Spawn Play)
        (:Update
          (Transformation|SetWorldScale3D (Variables|Default|GetWave) (Math|Vector|Lerp(Vector) "0, 0, 0" "0.750000,0.750000,0.750000" (Math|Float|Min(Float) _alpha _alpha_2))))
        (:Finished
          (if (< (.z (Transformation|GetWorldScale (Variables|Default|GetWave))) 0.1)
            (CallFunction|ClearSavedTransform)
            (Actor|DestroyActor)))))))

(event EventShow
  (Variables|Default|SetTargetSize "0.750000,0.750000,0.750000")
  (bind _alpha (Timeline|Timeline Play)
    (:Update
      (Transformation|SetWorldScale3D (Variables|Default|GetWave) (Math|Vector|Lerp(Vector) "0, 0, 0" (Variables|Default|GetTargetSize) _alpha)))))

(fn ConstructionScript)

(fn LineTrace
  (params (Start :type Vector) (End :type Vector))
  (bind (_outhit _returnvalue) (Collision|LineTraceByChannel (Math|Vector|MakeVector 1.05e+03 (.y Start) (.z Start)) (Math|Vector|MakeVector 1.05e+03 (.y End) (.z End)) "TraceTypeQuery3" false 0 "None"))
  (return (Math|Vector|MakeVector 975.0 (.y (.Location (Collision|BreakHitResult _outhit))) (.z (.Location (Collision|BreakHitResult _outhit)))) (.Normal (Collision|BreakHitResult _outhit)) _returnvalue))

(fn UpdateGameInstance
  (bind _returnvalue (Transformation|GetActorTransform))
  (bind _returnvalue_2 (Transformation|GetActorRightVector))
  (bind _gameinstance (Variables|Default|GetGameInstance))
  (CallFunction|ClearSavedTransform)
  (bind _returnvalue_3 (Game|GetCurrentLevelName true))
  (bind _output_get (Variables|Default|SetTag (Utilities|String|Append (Utilities|String|Append (Utilities|String|GetSubstring (Default|GetValuefromKey _gameinstance _returnvalue_3 (Variables|/Game/Game/Blueprints/GameInstance/BP_GameInstance.BP_GameInstance_C|GetLevelMap _gameinstance)) 0 4) "_" (Utilities|String|SelectString "0" "1" (!= (Utilities|Enum|Equal(Enum) (Utilities|String|GetSubstring (Default|GetValuefromKey _gameinstance _returnvalue_3 (Variables|/Game/Game/Blueprints/GameInstance/BP_GameInstance.BP_GameInstance_C|GetLevelMap _gameinstance)) 5) "0") (Variables|Rendering|GetbHidden)))) "Wave__" (Utilities|String|ToString(Integer) (Variables|Default|GetIndex)))))
  (Utilities|Map|Add (Variables|/Game/Game/Blueprints/GameInstance/BP_GameInstance.BP_GameInstance_C|GetTransformMap (Variables|Default|GetGameInstance)) _output_get (Math|Transform|SelectTransform (Math|Transform|MakeTransform (.location _returnvalue) (Math|Rotator|MakeRotfromZX (Transformation|GetActorUpVector) _returnvalue_2) (.scale _returnvalue)) (Math|Transform|MakeTransform (.location _returnvalue) (.rotation _returnvalue) (.scale _returnvalue)) (> (Math|Float|Absolute(Float) (Math|Vector|DotProduct _returnvalue_2 "1.000000,0.000000,0.000000")) 0.8))))

(fn ClearSavedTransform
  (bind _tag (Variables|Default|GetTag))
  (for _index (range 0 1)
    (Utilities|Map|Remove (Variables|/Game/Game/Blueprints/GameInstance/BP_GameInstance.BP_GameInstance_C|GetTransformMap (Variables|Default|GetGameInstance)) (Utilities|String|Append (Utilities|String|GetSubstring _tag 0 5) (Utilities|String|ToString(Integer) _index) (Utilities|String|GetSubstring _tag 6 7)))))