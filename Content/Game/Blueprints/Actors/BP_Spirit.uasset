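; BP_Spirit is a collectible spirit that trails the player once collected and can move to a lantern.
; On collection, a GameInstance event links it behind a spirit without a follower, forming a chain, or it follows the player.
; Tick eases it toward an offset behind its leader, aligned to the player's up vector.
; A FlipFlop-driven timeline toggles lantern mode, moving it to a target and switching custom depth rendering.
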(event Custom|CollectAnimation
  (Audio|PlaySoundatLocation "/Game/Game/Audio/SoundCues/SC_Spirit.SC_Spirit" (Transformation|GetActorLocation) "0, 0, 0" 1.0 1.0 0.0 0 0 0 0)
  (Default|CallFindTarget (Variables|Default|GetGameInstance) self)
  (Variables|Default|GetFollows
    (:then)
    (:else
      (Variables|Default|SetFollows (Game|GetPlayerCharacter 0)))))

(event Custom|ToggleLanternMode
  (params (TargetLocation :type Vector))
  (bind _spirit (Variables|Default|GetSpirit))
  (Utilities|FlowControl|FlipFlop
    (:A
      (Rendering|SetRenderCustomDepth _spirit false)
      (bind (_direction _alpha) (Timeline|Timeline Play)
        (:Update
          (Transformation|SetRelativeLocation (Variables|Default|GetSpirit) (Math|Vector|Lerp(Vector) "0.000000,0.000000,60.000000" "0.000000,-75.000000,60.000000" _alpha) false false)
          (switch Utilities|FlowControl|Switch|SwitchonETimelineDirection _direction
            (:Forward
              (Transformation|SetActorLocation (Math|Vector|Lerp(Vector) (Transformation|GetActorLocation) TargetLocation _alpha) false false))))))
    (:B
      (Rendering|SetRenderCustomDepth _spirit true)
      (Timeline|Timeline Reverse))))

(event Custom|SendTarget
  (params (Spirit :type BP%20Spirit%20Object%20Reference))
  (Variables|Default|GetFollows
    (:then
      (Variables|Default|GetFollowedBy
        (:then)
        (:else
          (Utilities|FlowControl|Delay 0.0)
          (Variables|BP_Spirit_C|SetFollows Spirit self)
          (Variables|Default|SetFollowedBy Spirit))))
    (:else)))

(event EventBeginPlay
  (EventDispatchers|BindEventtoCollectEvent (Variables|Default|GetBPC_Collectible) (delegate Custom|CollectAnimation))
  (bind _asbp_game_instance (Utilities|Casting|CastToBP_GameInstance (Game|GetGameInstance)))
  (bind _output_get (Variables|Default|SetGameInstance _asbp_game_instance))
  (EventDispatchers|BindEventtoFindTarget _output_get (delegate Custom|SendTarget))
  (Variables|/Game/Game/Blueprints/Components/BPC_Collectible.BPC_Collectible_C|SetIndex (Variables|Default|GetBPC_Collectible) (Variables|Default|GetIndex)))

(event EventTick
  (params (DeltaSeconds :type Float%20%28single-precision%29))
  (bind _returnvalue (Game|GetPlayerCharacter 0))
  (if (Variables|/Game/Game/Blueprints/Components/BPC_Collectible.BPC_Collectible_C|GetIsCollected (Variables|Default|GetBPC_Collectible))
    (bind _follows (Variables|Default|GetFollows)
      (:then
        (Utilities|IsValid _returnvalue
          (:Is%20Valid
            (Transformation|SetActorLocation (+ (Transformation|GetActorLocation) (Math|Vector|ClampVectorSize (/ (- (- (Transformation|GetActorLocation _follows) (Transformation|GetActorLocation)) (* (Math|Vector|GetRightVector (Variables|/Script/Engine.Character|GetMesh _returnvalue)) (* (Variables|/Game/Game/Blueprints/GameInstance/BP_GameInstance.BP_GameInstance_C|GetPlayerDirection (Variables|Default|GetGameInstance)) 75.0))) 1e+01) 0.0 1e+02)) false false)
            (Transformation|SetActorRotation (Math|Interpolation|RInterpTo (Transformation|GetActorRotation) (Math|Rotator|MakeRotfromZ (Math|Vector|GetUpVector (Variables|/Script/Engine.Character|GetMesh (Game|GetPlayerCharacter 0)))) DeltaSeconds 4.0)))))
      (:else))))

(fn ConstructionScript)

(fn ReturnRef
  (params (Lantern :type BP%20Lantern%20Object%20Reference))
  (Variables|/Game/Game/Blueprints/Actors/BP_Lantern.BP_Lantern_C|SetTempSpirit Lantern self)
  (return))