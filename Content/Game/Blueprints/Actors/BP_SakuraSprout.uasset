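; BP_SakuraSprout is a collectible sakura sprout actor that grows in when spawned and shrinks away when collected.
; Spawn plays a Timeline that scales the sprout from zero to three-quarter size.
; Interact calls OnCollect on BPCCollectible and plays a sound; the bound collect event reverses that Timeline, then destroys the actor after a short delay.
; The construction script initializes BPCInteractText with its child actor and box.
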(event Custom|CollectAnimation
  (Utilities|FlowControl|Sequence
    (:then_0
      (bind _alpha (Timeline|Timeline ReverseFromEnd)
        (:Update
          (Transformation|SetWorldScale3D (Variables|Default|GetSakuraSprout) (Math|Vector|Lerp(Vector) "0, 0, 0" "0.750000,0.750000,0.750000" _alpha)))))
    (:then_1
      (Utilities|FlowControl|Delay 0.25)
      (Actor|DestroyActor))))

(event Custom|Spawn
  (bind _alpha (Timeline|Timeline PlayFromStart)
    (:Update
      (Transformation|SetWorldScale3D (Variables|Default|GetSakuraSprout) (Math|Vector|Lerp(Vector) "0, 0, 0" "0.750000,0.750000,0.750000" _alpha)))))

(event EventBeginPlay
  (bind _asbp_game_instance (Utilities|Casting|CastToBP_GameInstance (Game|GetGameInstance)))
  (Variables|Default|SetGameInstance _asbp_game_instance)
  (EventDispatchers|BindEventtoCollectEvent (Variables|Default|GetBPC_Collectible) (delegate Custom|CollectAnimation)))

(event EventInteract
  (Default|OnCollect (Variables|Default|GetBPC_Collectible))
  (Audio|PlaySoundatLocation "/Game/Game/Audio/SoundCues/SC_Sakura.SC_Sakura" (Transformation|GetActorLocation) "0, 0, 0" 1.0 1.0 0.0 0 0 0 0))

(fn ConstructionScript
  (Default|InitializeDialogueStart (Variables|Default|GetBPC_InteractText) (Variables|Default|GetChildActor) (Variables|Default|GetBox)))