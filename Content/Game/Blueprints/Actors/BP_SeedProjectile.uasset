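; A seed projectile that plants a sakura sprout on the surface it hits.
; Each tick it moves along a manually integrated gravity arc, line-tracing ahead for impacts.
; Solid hits spawn a sprout aligned to the surface normal and record its tag and transform in the GameInstance.
; Hits on Water-tagged actors instead play a splash and add one to the Cherry score; either impact destroys the seed.
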(event EventTick
  (params (DeltaSeconds :type Float%20%28single-precision%29))
  (bind _returnvalue (Transformation|GetActorLocation))
  (bind (_outhit _returnvalue_2) (Collision|LineTraceByChannel _returnvalue (+ _returnvalue (* (Variables|Default|GetVelocity) DeltaSeconds)) "TraceTypeQuery3" false 0 "None"))
  (if _returnvalue_2
    (if (not (Actor|ActorHasTag (.HitActor (Collision|BreakHitResult _outhit)) "Water"))
      (Audio|SpawnSoundatLocation "/Game/Game/Audio/SoundCues/SC_Sakura.SC_Sakura" (.Location (Collision|BreakHitResult _outhit)) "0, 0, 0" 1.0 1.0 0.0 0 0)
      (bind _returnvalue_3 (Game|SpawnActorfromClass "/Game/Game/Blueprints/Actors/BP_SakuraSprout.BP_SakuraSprout_C" (Math|Transform|MakeTransform (.Location (Collision|BreakHitResult _outhit)) (Math|Rotator|MakeRotfromZX (.Normal (Collision|BreakHitResult _outhit)) (Math|Vector|MakeVector 1.0 0.0 0.0)) "0.750000,0.750000,0.750000") "Undefined" "MultiplyWithRoot" 0 0))
      (Variables|/Game/Game/Blueprints/Actors/BP_SakuraSprout.BP_SakuraSprout_C|SetGameInstance _returnvalue_3 (Variables|Default|GetGameInstance))
      (Variables|/Game/Game/Blueprints/Actors/BP_SakuraSprout.BP_SakuraSprout_C|SetIndex _returnvalue_3 (Utilities|Map|Length (Variables|/Game/Game/Blueprints/GameInstance/BP_GameInstance.BP_GameInstance_C|GetTransformMap (Variables|Default|GetGameInstance))))
      (Default|Spawn _returnvalue_3)
      (Default|MakeTag (Variables|/Game/Game/Blueprints/Actors/BP_SakuraSprout.BP_SakuraSprout_C|GetBPC_Collectible _returnvalue_3))
      (Utilities|Map|Add (Variables|/Game/Game/Blueprints/GameInstance/BP_GameInstance.BP_GameInstance_C|GetTransformMap (Variables|Default|GetGameInstance)) (Variables|/Game/Game/Blueprints/Components/BPC_Collectible.BPC_Collectible_C|GetTag (Variables|/Game/Game/Blueprints/Actors/BP_SakuraSprout.BP_SakuraSprout_C|GetBPC_Collectible _returnvalue_3)) (Math|Transform|MakeTransform (.Location (Collision|BreakHitResult _outhit)) (Math|Rotator|MakeRotfromZX (.Normal (Collision|BreakHitResult _outhit)) (Math|Vector|MakeVector 1.0 0.0 0.0)) "0.750000,0.750000,0.750000"))
      (Actor|DestroyActor)
      (else
        (Default|SetValue (Variables|Default|GetGameInstance) (Variables|/Game/Game/Blueprints/GameInstance/BP_GameInstance.BP_GameInstance_C|GetScoreMap (Variables|Default|GetGameInstance)) "Cherry" (+ (Default|GetScorefromMap (Variables|Default|GetGameInstance) "Cherry" (Variables|/Game/Game/Blueprints/GameInstance/BP_GameInstance.BP_GameInstance_C|GetScoreMap (Variables|Default|GetGameInstance))) 1))
        (Audio|SpawnSoundatLocation "/Game/Game/Audio/SoundCues/SC_Splash.SC_Splash" (Transformation|GetActorLocation) "0, 0, 0" 1.0 1.0 0.0 0 0)
        (Actor|DestroyActor)))
    (else
      (Transformation|SetActorLocation (+ _returnvalue (* (Variables|Default|GetVelocity) DeltaSeconds)) false false)
      (Variables|Default|SetVelocity (+ (* "0.000000,0.000000,-1150.000000" DeltaSeconds) (Variables|Default|GetVelocity))))))

(fn ConstructionScript)