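; BP_Bamboo is a bamboo actor that randomizes its own placement look, with no active gameplay logic.
; The Construction Script gives it a random yaw and a slight tilt from vertical using a random cone vector.
; It then randomly sinks and scales the static mesh to vary height and thickness.
; A CustomDepth variable controls whether the mesh renders to the custom depth pass.
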(event EventBeginPlay)

(event Collision|EventActorBeginOverlap
  (params (OtherActor :type Actor%20Object%20Reference)))

(event EventTick
  (params (DeltaSeconds :type Float%20%28single-precision%29)))

(fn ConstructionScript
  (bind _returnvalue (Math|Random|RandomFloatinRange 1e+01 2e+01))
  (bind _returnvalue_2 (Math|Random|RandomUnitVector))
  (bind _returnvalue_3 (Math|Vector2D|Normalize2D (Math|Vector2D|MakeVector2D (.x _returnvalue_2) (.y _returnvalue_2))))
  (Transformation|SetActorRotation (Math|Rotator|MakeRotfromZX (Math|Random|RandomUnitVectorinConeinDegrees "0.000000,0.000000,1.000000" 5.0) (Math|Vector|MakeVector (.x _returnvalue_3) (.y _returnvalue_3) 0.0)))
  (Transformation|SetRelativeLocation (Variables|Default|GetStaticMesh) (Math|Vector|MakeVector 0.0 0.0 (Math|Random|RandomFloatinRange 0.0 -1.5e+02)) false false)
  (Transformation|SetWorldScale3D (Variables|Default|GetStaticMesh) (Math|Vector|MakeVector _returnvalue _returnvalue (Math|Random|RandomFloatinRange 1e+01 15.0)))
  (Rendering|SetRenderCustomDepth (Variables|Default|GetStaticMesh) (Variables|Default|GetCustomDepth)))