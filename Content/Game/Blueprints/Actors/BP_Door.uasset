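; BP_Door is a level-exit double door that opens when both neighbouring sakura trees are active.
; On the GameInstance's SakuraActivate event, it briefly toggles sphere collision to gather tree states through BPI_SakuraTree overlaps.
; Two active trees get locked, and a Timeline slides the panels apart.
; A player inside the Box then triggers a white fade, spawn and lantern reset, and level transition; otherwise the door snaps shut.
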(event OnComponentBeginOverlap(Sphere)
  (params (OverlappedComponent :type Primitive%20Component%20Object%20Reference) (OtherActor :type Actor%20Object%20Reference) (OtherComp :type Primitive%20Component%20Object%20Reference) (OtherBodyIndex :type Integer) (bFromSweep :type Boolean) (SweepResult :type Hit%20Result%20Structure%20%28by%20ref%29))
  (if (Utilities|DoesObjectImplementInterface OtherActor "/Game/Game/Blueprints/Interfaces/BPI_SakuraTree.BPI_SakuraTree_C")
    (Utilities|Array|Add (Variables|Default|GetNeighbourSakura) OtherActor)
    (bind _hasflower (Class|BPISakuraTree|GetState(Message) OtherActor))
    (Utilities|Array|Add (Variables|Default|GetNeighbourSakuraState) _hasflower)))

(event Custom|TestNeighbourSakura
  (bind _array (Utilities|Array|MakeArray false false false false false false false))
  (bind _sphere (Variables|Default|GetSphere))
  (bind _gameinstance (Variables|Default|GetGameInstance))
  (bind _neighboursakurastate (Variables|Default|GetNeighbourSakuraState))
  (Utilities|Array|Clear (Variables|Default|GetNeighbourSakuraState))
  (Collision|SetCollisionEnabled _sphere "QueryOnly")
  (Collision|SetCollisionEnabled _sphere "NoCollision")
  (if (== (Utilities|Array|Length _neighboursakurastate) 2)
    (if (and (Utilities|Array|Get(acopy) _neighboursakurastate) (Utilities|Array|Get(acopy) _neighboursakurastate 1))
      (for _array_element (Variables|Default|GetNeighbourSakura)
        (Class|BPISakuraTree|Lock(Message) _array_element)
        (Utilities|FlowControl|Delay 1.0)
        (Components|Timeline|SetPlayRate (Variables|Default|GetTimeline) 1.0)
        (Audio|PlaySound2D "/Game/Game/Audio/SoundCues/SC_DoorOpen.SC_DoorOpen" 1.0 1.0 0.0 0 0)
        (bind (_direction _alpha) (Timeline|Timeline Play)
          (:Update
            (Utilities|FlowControl|Sequence
              (:then_0
                (Transformation|SetRelativeLocation (Variables|Default|GetLeftDoor) (Math|Vector|Lerp(Vector) "155.000000,5.000000,25.000000" "155.000000,-65.000000,25.000000" (Math|Float|Power _alpha 0.75)) false false))
              (:then_1
                (Transformation|SetRelativeLocation (Variables|Default|GetRightDoor) (Math|Vector|Lerp(Vector) "155.000000,5.000000,25.000000" "155.000000,75.000000,25.000000" (Math|Float|Power _alpha 0.75)) false false))))
          (:Finished
            (switch Utilities|FlowControl|Switch|SwitchonETimelineDirection _direction
              (:Forward
                (if (Collision|IsOverlappingActor (Variables|Default|GetBox) (Game|GetPlayerCharacter 0) :!class /Script/Engine.PrimitiveComponent)
                  (bind _returnvalue (UserInterface|CreateWidget "/Game/Game/Blueprints/Widgets/WBP_Fade.WBP_Fade_C" 0 "(R=1.000000,G=1.000000,B=1.000000,A=1.000000)" 0.25))
                  (Default|FadeOut _returnvalue)
                  (UserInterface|Viewport|AddtoViewport _returnvalue 0)
                  (Input|DisableInput (Game|GetPlayerCharacter 0) (Game|GetPlayerController 0))
                  (Variables|/Game/Game/Blueprints/GameInstance/BP_GameInstance.BP_GameInstance_C|SetSpawnPoint _gameinstance 0)
                  (Variables|/Game/Game/Blueprints/GameInstance/BP_GameInstance.BP_GameInstance_C|SetPastLanternState _gameinstance _array)
                  (Variables|/Game/Game/Blueprints/GameInstance/BP_GameInstance.BP_GameInstance_C|SetFutureLanternState _gameinstance _array)
                  (Audio|PlaySound2D "/Game/Game/Audio/SoundWaves/SW_Divine.SW_Divine" 1.0 1.0 0.0 0 0)
                  (Utilities|FlowControl|Delay 6.0)
                  (bind _returnvalue_2 (UserInterface|CreateWidget "/Game/Game/Blueprints/Widgets/WBP_LevelTransition.WBP_LevelTransition_C" 0 "(R=1.000000,G=1.000000,B=1.000000,A=1.000000)" (Variables|Default|GetText) (Variables|Default|GetLevelName) "(R=1.000000,G=1.000000,B=1.000000,A=1.000000)"))
                  (UserInterface|Viewport|AddtoViewport _returnvalue_2 0)
                  (else
                    (Components|Timeline|SetPlayRate (Variables|Default|GetTimeline) 12.0)
                    (Audio|PlaySound2D "/Game/Game/Audio/SoundCues/SC_DoorClose.SC_DoorClose" 1.0 1.0 0.0 0 0)
                    (Timeline|Timeline Reverse)))))))))))

(event EventBeginPlay
  (bind _asbp_game_instance (Utilities|Casting|CastToBP_GameInstance (Game|GetGameInstance)))
  (bind _output_get (Variables|Default|SetGameInstance _asbp_game_instance))
  (EventDispatchers|BindEventtoSakuraActivate _output_get (delegate Custom|TestNeighbourSakura)))

(fn ConstructionScript)