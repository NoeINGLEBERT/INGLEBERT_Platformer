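; Interactable gong actor that, when struck, plays a sound and sends out a pair of waves from its right and left spawn points.
; After a short delay it destroys previously tracked waves, spawns and indexes the new pair, and swings the gong mesh with a timeline.
; A binding to the GameInstance's wave persistence event adds those waves to the tracked list.
; The construction script initializes the interact text component.
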(event Custom|GetWave
  (params (Wave :type BP%20Wave%20Object%20Reference))
  (Utilities|Array|Add (Variables|Default|GetSpawnedWave) Wave))

(event EventBeginPlay
  (bind _asbp_game_instance (Utilities|Casting|CastToBP_GameInstance (Game|GetGameInstance)))
  (bind _output_get (Variables|Default|SetGameInstance _asbp_game_instance))
  (EventDispatchers|BindEventtoWavePersistence _output_get (delegate Custom|GetWave)))

(event EventInteract
  (bind _spawnedwave (Variables|Default|GetSpawnedWave))
  (Audio|PlaySoundatLocation "/Game/Game/Audio/SoundCues/SC_Gong.SC_Gong" (Transformation|GetActorLocation) "0, 0, 0" 1.0 1.0 0.0 0 0 0 0)
  (Utilities|FlowControl|Delay 0.15)
  (Utilities|FlowControl|Sequence
    (:then_0
      (for _array_element _spawnedwave
        (Utilities|IsValid _array_element
          (:Is%20Valid
            (Default|Destroy _array_element))))
      (Utilities|Array|Clear _spawnedwave)
      (for (_array_element_2 _array_index) (Utilities|Array|MakeArray (Transformation|GetWorldTransform (Variables|Default|GetSpawn%20Right)) (Transformation|GetWorldTransform (Variables|Default|GetSpawn%20Left)))
        (bind _returnvalue (Game|SpawnActorfromClass "/Game/Game/Blueprints/Actors/BP_Wave.BP_Wave_C" _array_element_2 "Undefined" "MultiplyWithRoot" 0 0))
        (Variables|/Game/Game/Blueprints/Actors/BP_Wave.BP_Wave_C|SetIndex _returnvalue _array_index)
        (Utilities|Array|Add (Variables|Default|GetSpawnedWave) _returnvalue)))
    (:then_1
      (bind _alpha (Timeline|GongAnimation PlayFromStart)
        (:Update
          (Transformation|SetRelativeRotation (Variables|Default|GetGong) (Math|Rotator|Lerp(Rotator) "0.000000,-90.000000,-90.000000" "0.000000,-90.000000,-120.000000" _alpha) false false))))))

(fn ConstructionScript
  (Default|InitializeDialogueStart (Variables|Default|GetBPC_InteractText) (Variables|Default|GetChildActor) (Variables|Default|GetBox)))