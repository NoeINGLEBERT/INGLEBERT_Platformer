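; Player for a side-view platformer that walks along surfaces of any orientation and dives into them with an inverse jump.
; Averaged line traces snap and align it to surfaces, while custom gravity pulls it back out of walls, then downward.
; Enhanced Input drives movement, interaction and mouse-aimed seed shots that spend Cherry score, with a traced arc preview.
; Overlaps handle landing, pickups and gates; WhiteMode swapping is marked unfinished.
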(event OnComponentEndOverlap(Sphere)
  (params (OverlappedComponent :type Primitive%20Component%20Object%20Reference) (OtherActor :type Actor%20Object%20Reference) (OtherComp :type Primitive%20Component%20Object%20Reference) (OtherBodyIndex :type Integer))
  (if (Variables|Default|GetWhiteMode)
    (if (and (!= OtherActor self) (Utilities|Array|IsEmpty (Collision|GetOverlappingActors (Variables|Default|GetSphere) "/Game/Game/Blueprints/Actors/BP_Wall.BP_Wall_C" :!class /Script/Engine.PrimitiveComponent)))
      (Variables|Default|SetGravityVector "0.000000,0.000000,-1.000000")
      (if (Variables|Default|GetIsInGround)
        (Variables|Default|SetIsInGround false)
        (Audio|PlaySoundatLocation "/Game/Game/Audio/SoundCues/SC_JumpOut.SC_JumpOut" (Transformation|GetWorldLocation (Variables|Character|GetMesh)) "0, 0, 0" 1.0 1.0 0.0 0 0 0 0)))))

(event OnComponentBeginOverlap(Sphere)
  (params (OverlappedComponent :type Primitive%20Component%20Object%20Reference) (OtherActor :type Actor%20Object%20Reference) (OtherComp :type Primitive%20Component%20Object%20Reference) (OtherBodyIndex :type Integer) (bFromSweep :type Boolean) (SweepResult :type Hit%20Result%20Structure%20%28by%20ref%29))
  (bind _returnvalue (Transformation|GetActorLocation))
  (Utilities|FlowControl|Sequence
    (:then_0
      (if (Variables|Default|GetWhiteMode)
        (if (and (not (Variables|Default|GetIsInGround)) (not (Variables|Default|GetIsOnGround)))
          (Utilities|Casting|CastToBP_Wall OtherActor)
          (Variables|Default|SetIsOnGround true)
          (Utilities|FlowControl|Delay 0.0)
          (Variables|Default|SetLocation "0, 0, 0")
          (Variables|Default|SetUpVector "0, 0, 0")
          (Variables|Default|SetHitNumber 0)
          (for _index (range 0 360)
            (bind (_outhit _returnvalue_2) (Collision|LineTraceByChannel _returnvalue (+ _returnvalue (* (Math|Vector|RotateVectorAroundAxis "0.000000,0.000000,1.000000" (Math|Conversions|ToFloat(Integer) _index) "1.000000,0.000000,0.000000") 6e+01)) "TraceTypeQuery3" false 0 "None"))
            (if _returnvalue_2
              (Variables|Default|SetHitNumber (+ (Variables|Default|GetHitNumber) 1))
              (Variables|Default|SetLocation (+ (Variables|Default|GetLocation) (.Location (Collision|BreakHitResult _outhit))))
              (Variables|Default|SetUpVector (+ (Variables|Default|GetUpVector) (.Normal (Collision|BreakHitResult _outhit))))))
          (Transformation|SetWorldLocation (Variables|Default|GetCone) (Math|Vector|Lerp(Vector) (Transformation|GetActorLocation) (/ (Variables|Default|GetLocation) (Variables|Default|GetHitNumber)) 0.5) false false)
          (Transformation|SetWorldRotation (Variables|Default|GetCone) (Math|Rotator|MakeRotfromZX (/ (Variables|Default|GetUpVector) (Variables|Default|GetHitNumber)) (Math|Vector|MakeVector 1.0 0.0 0.0)) false false)
          (Rendering|Material|SetScalarParameterValue (Variables|Default|GetDynamicMaterial) "ScaleZ" 1.0 :!class /Script/Engine.MaterialInstanceDynamic))))
    (:then_1
      (Default|TryCollect (Variables|Default|GetBPC_Collect) OtherActor))
    (:then_2
      (if (Utilities|DoesObjectImplementInterface OtherActor "/Game/Game/Blueprints/Interfaces/BPI_Gate.BPI_Gate_C")
        (Class|BPIGate|Enter(Message) OtherActor)))))

(event Custom|AutoMove
  (params (Input :type Vector%202D%20Structure))
  (Timeline|Timeline PlayFromStart
    (:Update
      (Utilities|Move (.x Input) (.y Input) :!label _label))
    (:Finished
      (goto _label Completed))))

(event Input|EnhancedActionEvents|EnhancedInputActionIA_Jump
  (params (ActionValue :type Boolean) (ElapsedSeconds :type Float%20%28double-precision%29) (TriggeredSeconds :type Float%20%28double-precision%29) (InputAction :type Input%20Action%20Object%20Reference :default "/Game/Game/Input/Actions/IA_Jump.IA_Jump"))
  (:Started
    (Utilities|InverseJump)))

(event Input|EnhancedActionEvents|EnhancedInputActionIA_Move
  (params (ActionValue :type Vector%202D%20Structure) (ElapsedSeconds :type Float%20%28double-precision%29) (TriggeredSeconds :type Float%20%28double-precision%29) (InputAction :type Input%20Action%20Object%20Reference :default "/Game/Game/Input/Actions/IA_Move.IA_Move"))
  (:Triggered
    (Utilities|Move (.x ActionValue) (.y ActionValue) :!label _label))
  (:Completed
    (goto _label Completed)))

(event Input|EnhancedActionEvents|EnhancedInputActionIA_Swap
  (params (ActionValue :type Boolean) (ElapsedSeconds :type Float%20%28double-precision%29) (TriggeredSeconds :type Float%20%28double-precision%29) (InputAction :type Input%20Action%20Object%20Reference :default "/Game/Game/Input/Actions/IA_Swap.IA_Swap"))
  ;[1 0 0] COMING SOON
  ; Ignorez les branchs White Mode, par défaut ils sont true
  (:Started
    (Variables|Default|SetWhiteMode (not (Variables|Default|GetWhiteMode)))))

(event Input|EnhancedActionEvents|EnhancedInputActionIA_Interact
  (params (ActionValue :type Boolean) (ElapsedSeconds :type Float%20%28double-precision%29) (TriggeredSeconds :type Float%20%28double-precision%29) (InputAction :type Input%20Action%20Object%20Reference :default "/Game/Game/Input/Actions/IA_Interact.IA_Interact"))
  (:Started
    (Utilities|Interact)))

(event Input|EnhancedActionEvents|EnhancedInputActionIA_Aim
  (params (ActionValue :type Boolean) (ElapsedSeconds :type Float%20%28double-precision%29) (TriggeredSeconds :type Float%20%28double-precision%29) (InputAction :type Input%20Action%20Object%20Reference :default "/Game/Game/Input/Actions/IA_Aim.IA_Aim"))
  (:Triggered
    (Utilities|Aim :!label _label))
  (:Completed
    (goto _label Completed)))

(event Input|EnhancedActionEvents|EnhancedInputActionIA_Shoot
  (params (ActionValue :type Boolean) (ElapsedSeconds :type Float%20%28double-precision%29) (TriggeredSeconds :type Float%20%28double-precision%29) (InputAction :type Input%20Action%20Object%20Reference :default "/Game/Game/Input/Actions/IA_Shoot.IA_Shoot"))
  (bind _gameinstance (Variables|Default|GetGameInstance))
  (:Started
    (Utilities|Shoot)
    (Default|CallUpdateScore _gameinstance "Cherry" (Default|GetScorefromMap _gameinstance "Cherry"))))

(event EventTick
  (params (DeltaSeconds :type Float%20%28single-precision%29))
  (bind _returnvalue (Transformation|GetActorLocation))
  (bind _mesh (Variables|Character|GetMesh))
  (bind _dynamicmaterial (Variables|Default|GetDynamicMaterial))
  (bind _gravityvector (Variables|Default|GetGravityVector))
  (bind _cone (Variables|Default|GetCone))
  (bind _cone_2 (Variables|Default|GetCone))
  (bind _mesh_2 (Variables|Character|GetMesh))
  (Variables|Default|SetDeltaTime (* DeltaSeconds 75.0))
  (if (Variables|/Game/Game/Blueprints/GameMode/BP_GameMode.BP_GameMode_C|GetInputEnabled (Variables|Default|GetGameMode))
    (Variables|/Game/Game/Blueprints/GameInstance/BP_GameInstance.BP_GameInstance_C|SetPlayerDirection (Variables|Default|GetGameInstance) (Math|Float|Sign(Float) (Variables|Default|GetHorizontalVelocity))))
  (if (Variables|Default|GetIsOnGround)
    (Variables|Default|SetLocation "0, 0, 0")
    (Variables|Default|SetUpVector "0, 0, 0")
    (Variables|Default|SetAllHit true)
    (for _index (range 0 50)
      (bind (_location _up_vector _returnvalue_2) (CallFunction|LineTrace (+ _returnvalue (* (Math|Vector|GetRightVector _cone) (- _index 25))) (+ (- _returnvalue (* (Math|Vector|GetUpVector _cone) 1e+02)) (* (Math|Vector|GetRightVector _cone) (- _index 25)))))
      (Variables|Default|SetLocation (+ _location (Variables|Default|GetLocation)))
      (Variables|Default|SetUpVector (+ _up_vector (Variables|Default|GetUpVector)))
      (Variables|Default|SetAllHit (and _returnvalue_2 (Variables|Default|GetAllHit))))
    (if (Variables|Default|GetAllHit)
      (Transformation|SetActorLocation (Math|Vector|Lerp(Vector) (Transformation|GetActorLocation) (/ (Variables|Default|GetLocation) 51.0) 0.5) false false)
      (Transformation|SetWorldLocation _cone_2 (Math|Vector|Lerp(Vector) (Transformation|GetActorLocation) (/ (Variables|Default|GetLocation) 51.0) 0.5) false false)
      (Transformation|SetWorldRotation _cone_2 (Math|Rotator|MakeRotfromZX (/ (Variables|Default|GetUpVector) 51.0) (Math|Vector|MakeVector 1.0 0.0 0.0)) false false)
      (if (not (Variables|Default|GetWhiteMode))
        (Transformation|SetWorldLocation (Variables|Character|GetMesh) (+ (Transformation|GetWorldLocation _mesh_2) (* (Math|Vector|GetUpVector _mesh_2) -102.0)) false false)
        (Transformation|SetWorldRotation _mesh (Math|Rotator|MakeRotfromZX (Math|Vector|NegateVector (Math|Vector|GetUpVector _mesh)) (Math|Vector|MakeVector 1.0 0.0 0.0)) false false)))
    (else
      (Variables|Default|SetVelocity (+ (Variables|Default|GetVelocity) (* (Variables|Default|GetGravityVector) (Variables|Default|GetDeltaTime))))
      (Transformation|SetActorLocation (+ (Transformation|GetActorLocation) (* (Variables|Default|GetVelocity) (Variables|Default|GetDeltaTime))) false false)
      (Transformation|SetWorldLocation (Variables|Character|GetMesh) (+ (Transformation|GetActorLocation) (* (Variables|Default|GetVelocity) (Variables|Default|GetDeltaTime))) false false)
      (Transformation|SetWorldRotation (Variables|Default|GetCone) (Math|Rotator|MakeRotfromZX (select (Variables|Default|GetIsInGround) _gravityvector (Math|Vector|NegateVector _gravityvector)) (Math|Vector|MakeVector 1.0 0.0 0.0)) false false)
      (bind _returnvalue_3 (Rendering|Material|GetScalarParameterValue _dynamicmaterial "ScaleZ" :!class /Script/Engine.MaterialInstanceDynamic))
      (Rendering|Material|SetScalarParameterValue _dynamicmaterial "ScaleZ" (Math|Float|Lerp _returnvalue_3 (Math|Float|SelectFloat -1.0 1.0 (Variables|Default|GetIsInGround)) 0.5) :!class /Script/Engine.MaterialInstanceDynamic))))

(event EventBeginPlay
  (bind _mesh (Variables|Character|GetMesh))
  (bind _asplayer_controller (Utilities|Casting|CastToPlayerController (Pawn|GetController)))
  (Utilities|IsValid (PlayerController|LocalPlayerSubsystems|GetEnhancedInputLocalPlayerSubsystem _asplayer_controller)
    (:Is%20Valid
      (Input|AddMappingContext (PlayerController|LocalPlayerSubsystems|GetEnhancedInputLocalPlayerSubsystem _asplayer_controller) "/Game/Game/Input/IMC_Default.IMC_Default" 0 "(bIgnoreAllPressedKeysUntilRelease=True,bForceImmediately=False,bNotifyUserSettings=False)")
      (bind _asbp_game_instance (Utilities|Casting|CastToBP_GameInstance (Game|GetGameInstance)))
      (Variables|Default|SetGameInstance _asbp_game_instance)
      (bind _asbp_game_mode (Utilities|Casting|CastToBP_GameMode (Game|GetGameMode)))
      (bind _output_get (Variables|Default|SetGameMode _asbp_game_mode))
      (Variables|/Game/Game/Blueprints/GameMode/BP_GameMode.BP_GameMode_C|SetPlayerRef _output_get self)
      (bind _returnvalue (Rendering|Material|CreateDynamicMaterialInstance _mesh 0 "/Game/Game/Materials/Surface/M_Player.M_Player" "None" :!class /Script/Engine.PrimitiveComponent))
      (bind _output_get_2 (Variables|Default|SetDynamicMaterial _returnvalue))
      (Rendering|Material|SetMaterial _mesh 0 _output_get_2))))

(fn ConstructionScript)

(fn LineTrace
  (params (Start :type Vector) (End :type Vector))
  (bind (_outhit _returnvalue) (Collision|LineTraceByChannel Start End "TraceTypeQuery3" false 0 "None"))
  (return (+ (Math|Vector|MakeVector 1.05e+03 (.y (.Location (Collision|BreakHitResult _outhit))) (.z (.Location (Collision|BreakHitResult _outhit)))) (* (.Normal (Collision|BreakHitResult _outhit)) 51.0)) (.Normal (Collision|BreakHitResult _outhit)) _returnvalue))

(fn GetMeshtoMouseVector
  (bind _returnvalue (Game|GetPlayerController 0))
  (bind _mesh (Variables|Character|GetMesh))
  (bind (_locationx _locationy) (Game|Player|GetMousePosition _returnvalue))
  (bind _returnvalue_2 (Transformation|GetWorldLocation _mesh))
  (bind _screenposition (Class|GameplayStatics|ProjectWorldtoScreen _returnvalue _returnvalue_2 false))
  (return (Math|Vector|Normalize (Math|Vector|MakeVector 0.0 (- _locationx (.x _screenposition)) (- (.y _screenposition) _locationy)))))