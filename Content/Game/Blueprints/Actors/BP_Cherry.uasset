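; Cherry collectible actor that delegates collection to its BPCCollectible component and handles the pickup feedback.
; On BeginPlay it binds CollectAnimation to the component's collect event, caches BP_GameInstance and, if that cast succeeds, passes its Index to the component.
; CollectAnimation plays the cherry sound and runs a timeline that shrinks the Cherry component to zero scale, then destroys the actor.
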(event Custom|CollectAnimation
  (Audio|SpawnSoundatLocation "/Game/Game/Audio/SoundWaves/SW_Cherry.SW_Cherry" (Transformation|GetActorLocation) "0, 0, 0" 1.0 1.0 0.0 0 0)
  (bind _alpha (Timeline|Timeline PlayFromStart)
    (:Update
      (Transformation|SetWorldScale3D (Variables|Default|GetCherry) (Math|Vector|Lerp(Vector) "0.500000,0.500000,0.500000" "0, 0, 0" _alpha)))
    (:Finished
      (Actor|DestroyActor))))

(event EventBeginPlay
  (EventDispatchers|BindEventtoCollectEvent (Variables|Default|GetBPC_Collectible) (delegate Custom|CollectAnimation))
  (bind _asbp_game_instance (Utilities|Casting|CastToBP_GameInstance (Game|GetGameInstance)))
  (Variables|Default|SetGameInstance _asbp_game_instance)
  (Variables|/Game/Game/Blueprints/Components/BPC_Collectible.BPC_Collectible_C|SetIndex (Variables|Default|GetBPC_Collectible) (Variables|Default|GetIndex)))

(fn ConstructionScript)