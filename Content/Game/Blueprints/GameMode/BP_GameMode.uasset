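; Game mode that sets up each level on BeginPlay: HUD, screen fade, player spawn and world state persisted in BP_GameInstance.
; It refills lanterns from past/future states and respawns cherries, sakura sprouts, spirits and waves by parsing TransformMap keys encoding level, type and index.
; Sprouts from a paired level can appear as trees, and collected spirits form a linked follower chain behind the player.
; FadeOutMusic drives music volume through a timeline.
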(event Custom|FadeOutMusic
  (bind _alpha (Timeline|Timeline PlayFromStart)
    (:Update
      (Audio|Components|Audio|SetVolumeMultiplier (Variables|/Game/Game/Blueprints/GameInstance/BP_GameInstance.BP_GameInstance_C|GetMusic (Variables|Default|GetGameInstance)) _alpha :!class /Script/Engine.AudioComponent))))

(event EventBeginPlay
  (bind _returnvalue (Game|GetPlayerCharacter 0))
  (bind _returnvalue_2 (Game|GetPlayerCharacter 0))
  (bind _returnvalue_3 (Transformation|GetActorTransform _returnvalue))
  (bind _returnvalue_4 (Transformation|GetActorTransform _returnvalue_2))
  (bind _asbp_game_instance (Utilities|Casting|CastToBP_GameInstance (Game|GetGameInstance)))
  (bind _output_get (Variables|Default|SetGameInstance _asbp_game_instance))
  (Default|CallInitialize _output_get)
  (bind _returnvalue_5 (Game|GetCurrentLevelName true))
  (Utilities|Array|AddUnique (Variables|/Game/Game/Blueprints/GameInstance/BP_GameInstance.BP_GameInstance_C|GetInitializedLevel (Variables|Default|GetGameInstance)) _returnvalue_5)
  (bind _returnvalue_6 (UserInterface|CreateWidget "/Game/Game/Blueprints/Widgets/WBP_HUD.WBP_HUD_C"))
  (UserInterface|Viewport|AddtoViewport _returnvalue_6 0)
  (bind _returnvalue_7 (UserInterface|CreateWidget "/Game/Game/Blueprints/Widgets/WBP_Fade.WBP_Fade_C"))
  (UserInterface|Viewport|AddtoViewport _returnvalue_7 0)
  (Default|Fadein _returnvalue_7)
  (Input|DisableInput (Game|GetPlayerCharacter 0) (Game|GetPlayerController 0))
  (Utilities|FlowControl|Delay 0.2)
  (Default|CallSpawnPlayer (Variables|/Game/Game/Blueprints/GameInstance/BP_GameInstance.BP_GameInstance_C|GetSpawnPoint (Variables|Default|GetGameInstance)))
  (Utilities|FlowControl|Delay 0.2)
  (Utilities|FlowControl|Sequence
    (:then_0
      (for (_array_element _array_index) (Variables|Default|GetLanterns)
        (bind _returnvalue_8 (Game|GetCurrentLevelName true))
        (bind _keys (Utilities|Map|Keys (Variables|/Game/Game/Blueprints/GameInstance/BP_GameInstance.BP_GameInstance_C|GetLevelMap (Variables|Default|GetGameInstance))))
        (if (Utilities|Array|Get(acopy) (select (== (Utilities|Array|FindItem _keys _returnvalue_8) 0) (Variables|/Game/Game/Blueprints/GameInstance/BP_GameInstance.BP_GameInstance_C|GetPastLanternState (Variables|Default|GetGameInstance)) (Variables|/Game/Game/Blueprints/GameInstance/BP_GameInstance.BP_GameInstance_C|GetFutureLanternState (Variables|Default|GetGameInstance))) _array_index)
          (bind _returnvalue_9 (Game|SpawnActorfromClass "/Game/Game/Blueprints/Actors/BP_Spirit.BP_Spirit_C" (Math|Transform|MakeTransform (Transformation|GetWorldLocation (Variables|/Game/Game/Blueprints/Actors/BP_Lantern.BP_Lantern_C|GetAnchorPoint _array_element)) "0, 0, 0" "1.000000,1.000000,1.000000") "Undefined" "MultiplyWithRoot" 0 0))
          (bind _output_get_2 (Variables|/Game/Game/Blueprints/Actors/BP_Lantern.BP_Lantern_C|SetSpirit _array_element _returnvalue_9))
          (Default|ToggleLanternMode _output_get_2 (Transformation|GetActorLocation _returnvalue_9))
          (Variables|/Game/Game/Blueprints/Components/BPC_Collectible.BPC_Collectible_C|SetIsCollected (Variables|/Game/Game/Blueprints/Actors/BP_Spirit.BP_Spirit_C|GetBPC_Collectible _output_get_2) true))))
    (:then_1
      (bind _returnvalue_10 (Game|GetCurrentLevelName true))
      (Variables|Default|SetCurrentLevel (Default|GetValuefromKey (Variables|Default|GetGameInstance) _returnvalue_10 (Variables|/Game/Game/Blueprints/GameInstance/BP_GameInstance.BP_GameInstance_C|GetLevelMap (Variables|Default|GetGameInstance))))
      (for _index (range 0 (- (Utilities|Map|Length (Variables|/Game/Game/Blueprints/GameInstance/BP_GameInstance.BP_GameInstance_C|GetTransformMap (Variables|Default|GetGameInstance))) 1))
        (bind _keys_2 (Utilities|Map|Keys (Variables|/Game/Game/Blueprints/GameInstance/BP_GameInstance.BP_GameInstance_C|GetTransformMap (Variables|Default|GetGameInstance))))
        (Variables|Default|SetTargetLevel (Utilities|String|GetSubstring (Utilities|Array|Get(acopy) _keys_2 _index) 0 6))
        (bind _values (Utilities|Map|Values (Variables|/Game/Game/Blueprints/GameInstance/BP_GameInstance.BP_GameInstance_C|GetTransformMap (Variables|Default|GetGameInstance))))
        (switch string (Utilities|String|GetSubstring (Utilities|Array|Get(acopy) _keys_2 _index) 6 6)
          (:Cherry
            (if (Utilities|Enum|Equal(Enum) (Variables|Default|GetTargetLevel) (Variables|Default|GetCurrentLevel))
              (bind _returnvalue_11 (Game|SpawnActorfromClass "/Game/Game/Blueprints/Actors/BP_Cherry.BP_Cherry_C" (Utilities|Array|Get(acopy) _values _index) "Undefined" "MultiplyWithRoot" 0 0))
              (bind _output_get_3 (Variables|/Game/Game/Blueprints/Actors/BP_Cherry.BP_Cherry_C|SetIndex _returnvalue_11 (Math|Conversions|ToInteger(Byte) (Utilities|String|GetSubstring (Utilities|Array|Get(acopy) _keys_2 _index) 12 10))))
              (Variables|/Game/Game/Blueprints/Components/BPC_Collectible.BPC_Collectible_C|SetIndex (Variables|/Game/Game/Blueprints/Actors/BP_Cherry.BP_Cherry_C|GetBPC_Collectible _returnvalue_11) _output_get_3)))
          (:Sakura
            (if (Utilities|Enum|Equal(Enum) (Variables|Default|GetTargetLevel) (Variables|Default|GetCurrentLevel))
              (bind _returnvalue_12 (Game|SpawnActorfromClass "/Game/Game/Blueprints/Actors/BP_SakuraSprout.BP_SakuraSprout_C" (Utilities|Array|Get(acopy) _values _index) "Undefined" "MultiplyWithRoot" 0 0))
              (bind _output_get_4 (Variables|/Game/Game/Blueprints/Actors/BP_SakuraSprout.BP_SakuraSprout_C|SetIndex _returnvalue_12 (Math|Conversions|ToInteger(Byte) (Utilities|String|GetSubstring (Utilities|Array|Get(acopy) _keys_2 _index) 12 10))))
              (Variables|/Game/Game/Blueprints/Components/BPC_Collectible.BPC_Collectible_C|SetIndex (Variables|/Game/Game/Blueprints/Actors/BP_SakuraSprout.BP_SakuraSprout_C|GetBPC_Collectible _returnvalue_12) _output_get_4)
              (elif (and (Utilities|Enum|Equal(Enum) (Utilities|String|GetSubstring (Variables|Default|GetTargetLevel) 0 4) (Utilities|String|GetSubstring (Variables|Default|GetCurrentLevel) 0 4)) (Utilities|Enum|Equal(Enum) (Utilities|String|GetSubstring (Variables|Default|GetCurrentLevel) 5) "1"))
                (Game|SpawnActorfromClass "/Game/Game/Blueprints/Actors/BP_SakuraTree.BP_SakuraTree_C" (Utilities|Array|Get(acopy) _values _index) "Undefined" "MultiplyWithRoot" 0 0))))
          (:Spirit
            (if (Utilities|Enum|Equal(Enum) (Variables|Default|GetTargetLevel) (Variables|Default|GetCurrentLevel))
              (bind _returnvalue_13 (Game|SpawnActorfromClass "/Game/Game/Blueprints/Actors/BP_Spirit.BP_Spirit_C" (Utilities|Array|Get(acopy) _values _index) "Undefined" "MultiplyWithRoot" 0 0))
              (bind _output_get_5 (Variables|/Game/Game/Blueprints/Actors/BP_Spirit.BP_Spirit_C|SetIndex _returnvalue_13 (Math|Conversions|ToInteger(Byte) (Utilities|String|GetSubstring (Utilities|Array|Get(acopy) _keys_2 _index) 12 10))))
              (Variables|/Game/Game/Blueprints/Components/BPC_Collectible.BPC_Collectible_C|SetIndex (Variables|/Game/Game/Blueprints/Actors/BP_Spirit.BP_Spirit_C|GetBPC_Collectible _returnvalue_13) _output_get_5)))
          (:Wave__
            (bind _returnvalue_14 (Game|SpawnActorfromClass "/Game/Game/Blueprints/Actors/BP_Wave.BP_Wave_C" (Utilities|Array|Get(acopy) _values _index) "Undefined" "MultiplyWithRoot" 0 0))
            (Variables|/Game/Game/Blueprints/Actors/BP_Wave.BP_Wave_C|SetIndex _returnvalue_14 (Math|Conversions|ToInteger(Byte) (Utilities|String|GetSubstring (Utilities|Array|Get(acopy) _keys_2 _index) 12 10)))
            (Variables|/Game/Game/Blueprints/Actors/BP_Wave.BP_Wave_C|SetTag _returnvalue_14 (Utilities|Array|Get(acopy) _keys_2 _index))
            (Rendering|SetActorHiddenInGame _returnvalue_14 (Utilities|Enum|NotEqual(Enum) (Variables|Default|GetTargetLevel) (Variables|Default|GetCurrentLevel)))
            (Default|CallWavePersistence (Variables|Default|GetGameInstance) _returnvalue_14)))))
    (:then_2
      (if (> (Default|GetScorefromMap (Variables|Default|GetGameInstance) "Spirit" (Variables|/Game/Game/Blueprints/GameInstance/BP_GameInstance.BP_GameInstance_C|GetScoreMap (Variables|Default|GetGameInstance))) 0)
        (bind _returnvalue_15 (Game|SpawnActorfromClass "/Game/Game/Blueprints/Actors/BP_Spirit.BP_Spirit_C" (Math|Transform|MakeTransform (- (.location _returnvalue_4) "0.000000,150.000000,0.000000") (.rotation _returnvalue_4) (.scale _returnvalue_4)) "Undefined" "MultiplyWithRoot" 0 0))
        (Variables|/Game/Game/Blueprints/Components/BPC_Collectible.BPC_Collectible_C|SetIsCollected (Variables|/Game/Game/Blueprints/Actors/BP_Spirit.BP_Spirit_C|GetBPC_Collectible _returnvalue_15) true)
        (bind _output_get_6 (Variables|Default|SetTempSpirit _returnvalue_15))
        (Variables|/Game/Game/Blueprints/Actors/BP_Spirit.BP_Spirit_C|SetFollows _output_get_6 _returnvalue_2)
        (if (> (Default|GetScorefromMap (Variables|Default|GetGameInstance) "Spirit" (Variables|/Game/Game/Blueprints/GameInstance/BP_GameInstance.BP_GameInstance_C|GetScoreMap (Variables|Default|GetGameInstance))) 1)
          (for _index_2 (range 1 (- (Default|GetScorefromMap (Variables|Default|GetGameInstance) "Spirit" (Variables|/Game/Game/Blueprints/GameInstance/BP_GameInstance.BP_GameInstance_C|GetScoreMap (Variables|Default|GetGameInstance))) 1))
            (bind _returnvalue_16 (Game|SpawnActorfromClass "/Game/Game/Blueprints/Actors/BP_Spirit.BP_Spirit_C" (Math|Transform|MakeTransform (- (.location _returnvalue_3) "0.000000,150.000000,0.000000") (.rotation _returnvalue_3) (.scale _returnvalue_3)) "Undefined" "MultiplyWithRoot" 0 0))
            (Variables|/Game/Game/Blueprints/Components/BPC_Collectible.BPC_Collectible_C|SetIsCollected (Variables|/Game/Game/Blueprints/Actors/BP_Spirit.BP_Spirit_C|GetBPC_Collectible _returnvalue_16) true)
            (Variables|/Game/Game/Blueprints/Actors/BP_Spirit.BP_Spirit_C|SetFollowedBy (Variables|Default|GetTempSpirit) _returnvalue_16)
            (Variables|/Game/Game/Blueprints/Actors/BP_Spirit.BP_Spirit_C|SetFollows _returnvalue_16 (Variables|Default|GetTempSpirit))
            (Variables|Default|SetTempSpirit _returnvalue_16)))))))

(fn ConstructionScript)